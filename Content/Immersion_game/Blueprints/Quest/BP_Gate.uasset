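; BP_Gate is a key-locked, interactable double gate that opens with a short cutscene.
; Focus toggles a tooltip widget and custom-depth outline on both doors until used.
; Interaction tries the key through BPC_MiniInventory, showing a temporary closed-door widget on failure.
; On success it moves the input-disabled player into position, blends to the gate's view, and uses timers, a montage and a rotation timeline before restoring control.
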(event `self.ReceiveBeginPlay`
  (`Widget.SetVisibility` (`WidgetComponent.GetWidget` (`self.BP_WidgetComp`)) "Collapsed"))

(event `/Game/Immersion_game/Blueprints/Interfaces/BPI_Interact.CancelCanInteract`
  (`self.ActivateOutlinerAndTooltip` false)
  (bind _newvar (`self.NewVar`)
    (:`then`
      (`Widget.RemoveFromParent` _newvar))
    (:`else`)))

(event `Open`
  (bind _relative_rotation1 (`self.Relative Rotation1`))
  (bind _relative_rotation (`self.Relative Rotation`))
  (`/Engine/EditorBlueprintResources/StandardMacros.DoOnce` false
    (:`Completed`
      (set `self.Relative Rotation1` (`SceneComponent.RelativeRotation` (`self.GateDoor1`)))
      (set `self.Relative Rotation` (`SceneComponent.RelativeRotation` (`self.GateDoor`)))
      (bind (_direction _alpha) (`Timeline|Timeline` :!via `PlayFromStart`)
        (:`Update`
          (`SceneComponent.K2_SetRelativeRotation` (`self.GateDoor`) (`KismetMathLibrary.RLerp` _relative_rotation (`KismetMathLibrary.ComposeRotators` _relative_rotation (struct :`Yaw` 60.0)) _alpha true) false false)
          (`SceneComponent.K2_SetRelativeRotation` (`self.GateDoor1`) (`KismetMathLibrary.RLerp` _relative_rotation1 (`KismetMathLibrary.ComposeRotators` _relative_rotation1 (struct :`Yaw` -60.0)) _alpha true) false false))
        (:`Finished`
          (`self.EndCutscene`))))))

(event `CustomEvent`
  (`KismetSystemLibrary.Delay` 2.0)
  (bind _newvar (`self.NewVar`)
    (:`then`
      (`Widget.RemoveFromParent` _newvar))
    (:`else`)))

(fn `ActivateOutlinerAndTooltip`
  (params (Active :type Boolean))
  (bind _returnvalue (and (not (`self.Used`)) Active))
  (`Widget.SetVisibility` (`WidgetComponent.GetWidget` (`self.BP_WidgetComp`)) (select `bool` _returnvalue :`false` "Collapsed" :`true` "Visible" :!type "ESlateVisibility Enum"))
  (`PrimitiveComponent.SetRenderCustomDepth` (`self.GateDoor1`) _returnvalue)
  (`PrimitiveComponent.SetRenderCustomDepth` (`self.GateDoor`) _returnvalue))

(fn `CanInteract`
  (params (Hit :type "HitResult Structure") (QueryFromActor :type "Actor Object Reference"))
  (returns (True :type Boolean))
  (`self.ActivateOutlinerAndTooltip` true)
  (return true))

(fn `EndCutscene`
  (`PlayerController.SetViewTargetWithBlend` (`GameplayStatics.GetPlayerController` 0) (`GameplayStatics.GetPlayerCharacter` 0) 1.0 "VTBlend_Linear" 1.0 false)
  (`self.EnableInput` (`GameplayStatics.GetPlayerCharacter` 0) (`GameplayStatics.GetPlayerController` 0)))

(fn `Move and Rotate Character`
  (bind _returnvalue (`GameplayStatics.GetPlayerController` 0))
  (bind _characterposition (`self.CharacterPosition`))
  (`AIBlueprintHelperLibrary.SimpleMoveToLocation` _returnvalue (`SceneComponent.K2_GetComponentLocation` _characterposition))
  (`Controller.SetControlRotation` _returnvalue (`SceneComponent.K2_GetComponentRotation` _characterposition)))

(fn `PlayAnimation`
  (bind _montagelengtgh (`/Game/Immersion_game/Core/Character/BP_Character.PlayMontage` (cast `/Game/Immersion_game/Core/Character/BP_Character` (`GameplayStatics.GetPlayerCharacter` 0) :!pure true) "/Game/Resources/Animations/Hero/Opening_Montage.Opening_Montage" 1.0 false))
  (`KismetSystemLibrary.K2_SetTimerDelegate` (`|CreateDelegate` :!event `Open`) 0.01 false _montagelengtgh))

(fn `StartInteract`
  (params (InteractByActor :type "Actor Object Reference"))
  (returns (bSuccess :type Boolean) (bShouldPlayAnim :type Boolean) (bShouldRotateCharacterToObject :type Boolean))
  (bind _bsuccess (`/Game/Immersion_game/Blueprints/Components/MiniInventrory/BPC_MiniInventory.TryUseItem` (`self.GetComponentByClass` InteractByActor "/Game/Immersion_game/Blueprints/Components/MiniInventrory/BPC_MiniInventory.BPC_MiniInventory_C") (`self.KeyRowName`)))
  (if _bsuccess
    (`self.DisableInput` (`GameplayStatics.GetPlayerCharacter` 0) (`GameplayStatics.GetPlayerController` 0))
    (set `self.Used` true)
    (`self.Move and Rotate Character`)
    (`PlayerController.SetViewTargetWithBlend` (`GameplayStatics.GetPlayerController` 0) self 1.0 "VTBlend_Linear" 1.0 false)
    (`KismetSystemLibrary.K2_SetTimerDelegate` (`|CreateDelegate` :!event `PlayAnimation`) 0.01 false 1.0)
    (set `self.Used` true)
    (`self.ActivateOutlinerAndTooltip` false)
    (return true false false)
    (else
      (bind _returnvalue (`|CreateWidget` "/Game/Immersion_game/UI/Service/W_DoorClose.W_DoorClose_C"))
      (set `self.NewVar` _returnvalue)
      (`UserWidget.AddToViewport` _returnvalue 0)
      (`self.CustomEvent`))))

(fn `UserConstructionScript`)