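; Base component that holds a float value between zero and a maximum, with functions to set, increase, decrease and query it.
; It starts full, and increases and decreases pass through SetValue, which clamps the result and fires change, full and zero notifications.
; Increase and decrease also fire their own notifications.
; Tick is enabled only by the ShowDebug flag and prints the current state.
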(event `self.ReceiveBeginPlay`
  (set `self.FloatValue` (`KismetMathLibrary.FClamp` (`self.MaxFloatValue`) 0.0 (`self.MaxFloatValue`)))
  (`self.OnChangeValue` (`self.FloatValue`))
  (`self.SetComponentTickEnabled` (`self.bShowDebug`)))

(event `self.ReceiveTick`
  (params (DeltaSeconds :type "Float (single-precision)"))
  (`self.ShowDebug`))

(fn `DecreaseValue`
  (params (DecreaseValue :type "Float (double-precision)"))
  (`self.SetValue` (- (`self.FloatValue`) (`KismetMathLibrary.FMin` (`KismetMathLibrary.FMax` (`local.DecreaseValue`)) (`self.FloatValue`))))
  (`self.OnDecreaseValue` (`self.FloatValue`)))

(fn `GetValue`
  (returns (FloatValue :type "Float (double-precision)"))
  (return (`self.FloatValue`)))

(fn `GetValueEqualZero`
  (returns (bEqualZero :type Boolean))
  (return (<= (`self.FloatValue`) 0.0)))

(fn `GetValueFull`
  (returns (bFull :type Boolean))
  (return (>= (`self.FloatValue`) (`self.MaxFloatValue`))))

(fn `IncreaseValue`
  (params (IncreaseValue :type "Float (double-precision)"))
  (`self.SetValue` (+ (`KismetMathLibrary.FMin` (`local.IncreaseValue`) (- (`self.MaxFloatValue`) (`self.FloatValue`))) (`self.FloatValue`)))
  (`self.OnIncreaseValue` (`self.FloatValue`)))

(fn `SetValue`
  (params (FloatValue :type "Float (double-precision)"))
  (locals (LocalFloatValue :type "Float (double-precision)" :default 0.0))
  (bind _maxfloatvalue (`self.MaxFloatValue`))
  (set `local.LocalFloatValue` (`KismetMathLibrary.FClamp` FloatValue 0.0 (`self.MaxFloatValue`)))
  (if (and (!= (`self.FloatValue`) _maxfloatvalue) (== _maxfloatvalue (`local.LocalFloatValue`)))
    (`self.OnFullValue`)
    (elif (and (== (`local.LocalFloatValue`) 0.0) (!= (`self.FloatValue`) 0.0))
      (`self.OnZeroValue`)))
  (set `self.FloatValue` (`local.LocalFloatValue`))
  (`self.OnChangeValue` (`self.FloatValue`)))

(fn `ShowDebug`
  (`KismetSystemLibrary.PrintString` (`KismetTextLibrary.Conv_TextToString` (`|FormatText` "From BPC_BaseFloatComponentDebug \nMaxValue : {MaxValue} \nCurrent Value : {CurrentValue} \nValueEqualZero : {VEZ}" (`self.MaxFloatValue`) (`self.FloatValue`) (`self.GetValueEqualZero`))) true true (struct :`R` 0.021003 :`G` 1.0 :`A` 1.0) 0.0))