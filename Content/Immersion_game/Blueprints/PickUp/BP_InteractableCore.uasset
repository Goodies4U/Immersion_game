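; Base Blueprint for interactable objects, with a highlight and widget prompt shown while interaction is available.
; CanInteract always returns true, enabling custom depth on the Interactable component and showing the widget; CancelCanInteract reverses both.
; StartInteract calls CanInteract, then InteractLogic, passing back success plus animation and character-rotation flags.
; InteractLogic is a stub returning all false, apparently for child classes to override, and the widget starts collapsed on BeginPlay.
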(event `self.ReceiveBeginPlay`
  (`self.ToggleInteractFX` false))

(event `self.CancelCanInteract`
  (`PrimitiveComponent.SetRenderCustomDepth` (`self.Interactable`) false)
  (`self.ToggleInteractFX` false))

(fn `CanInteract`
  (params (Hit :type "HitResult Structure") (QueryFromActor :type "Actor Object Reference"))
  (returns (True :type Boolean))
  (`PrimitiveComponent.SetRenderCustomDepth` (`self.Interactable`) true)
  (`self.ToggleInteractFX` true)
  (return true))

(fn `InteractLogic`
  (params (InteractByActor :type "Actor Object Reference"))
  (returns (bSuccess :type Boolean) (bShouldPlayAnim :type Boolean) (bShouldRotateCharacterToObject :type Boolean))
  (return false false false))

(fn `StartInteract`
  (params (InteractByActor :type "Actor Object Reference"))
  (returns (bSuccess :type Boolean) (bShouldPlayAnim :type Boolean) (bShouldRotateCharacterToObject :type Boolean))
  (bind _true (`self.CanInteract` (struct) InteractByActor))
  (if _true
    (bind (_bsuccess _bshouldplayanim _bshouldrotatecharactertoobject) (`self.InteractLogic` InteractByActor))
    (if _bsuccess
      (return true _bshouldplayanim _bshouldrotatecharactertoobject)
      (else
        _)))
  (return false false false))

(fn `ToggleInteractFX`
  (params (bToggle :type Boolean))
  (bind _bp_widgetcomp (`self.BP_WidgetComp`))
  (bind _returnvalue (`WidgetComponent.GetWidget` _bp_widgetcomp))
  (`/Engine/EditorBlueprintResources/StandardMacros.IsValid` _bp_widgetcomp
    (:`Is Valid`
      (`/Engine/EditorBlueprintResources/StandardMacros.IsValid` _returnvalue
        (:`Is Valid`
          (`Widget.SetVisibility` _returnvalue (select `bool` bToggle :`false` "Collapsed" :`true` "Visible" :!type "ESlateVisibility Enum")))))))

(fn `UserConstructionScript`)