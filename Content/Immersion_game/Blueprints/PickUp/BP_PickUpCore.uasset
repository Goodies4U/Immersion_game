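; Base pickup actor that can be highlighted, interacted with and removed from the world on use.
; The construction script sets its mesh from the ItemInfo data table row, clearing it when the row or model is missing.
; CanInteract always succeeds and enables custom depth on the mesh, which CancelCanInteract disables.
; StartInteract calls CanInteract, runs the empty PickUpLogic hook, then destroys the actor.
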(event `self.ReceiveBeginPlay`)

(event `self.CancelCanInteract`
  (`PrimitiveComponent.SetRenderCustomDepth` (`self.PickUpCore`) false))

(event `PickUpLogic`)

(fn `CanInteract`
  (returns (True :type Boolean))
  (`PrimitiveComponent.SetRenderCustomDepth` (`self.PickUpCore`) true)
  (return true))

(fn `StartInteract`
  (returns (bSuccess :type Boolean))
  (bind _true (`self.CanInteract`))
  (if _true
    (`self.PickUpLogic`)
    (`self.K2_DestroyActor`)
    (return true)
    (else
      (return false))))

(fn `UserConstructionScript`
  (bind (_iteminfo_datatable _iteminfo_rowname) (break `DataTableRowHandle` (`self.ItemInfo`)))
  (bind _pickupcore (`self.PickUpCore`))
  (`/Engine/EditorBlueprintResources/StandardMacros.IsValid` _iteminfo_datatable
    (:`Is Valid`
      (bind _returnvalue (`|GetDataTableRow` _iteminfo_datatable _iteminfo_rowname)
        (:`then`
          (bind ((`Model_12_610D90534B2005F60D932E9BF72B2F54` _model)) (break `/Game/Immersion_game/Blueprints/PickUp/PickUpInfo/S_ItemInfo` _returnvalue))
          (`/Engine/EditorBlueprintResources/StandardMacros.IsValid` _model
            (:`Is Valid`
              (`StaticMeshComponent.SetStaticMesh` _pickupcore _model))
            (:`Is Not Valid`
              (`StaticMeshComponent.SetStaticMesh` _pickupcore null :!label _label))))
        (:`RowNotFound`
          (goto _label))))))