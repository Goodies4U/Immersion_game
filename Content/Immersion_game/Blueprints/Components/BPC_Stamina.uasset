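; Stamina component that drains while the owning character runs and regenerates after running stops, built on a parent value component.
; Looping timers drive drain and delayed refresh, with the drain timer paused on stop or cleared when exhausted.
; Drain applies only above run speed and outside of falling.
; A rest flag, updated during refresh, blocks running below a threshold and fires a start-rest event.
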(event `self.ReceiveBeginPlay`
  (`parent.ReceiveBeginPlay`)
  (add `self.OnZeroValue` (`|CreateDelegate` :!event `StartRefresh`))
  (add `self.OnFullValue` (`|CreateDelegate` :!event `StopRefresh`)))

(fn `GetCanRun`
  (returns (bCanRun :type Boolean))
  (return (and (not (`self.bNeedRest`)) (> (`self.GetValue`) 0.0))))

(fn `GetNeedRest`
  (returns (bNeedRest :type Boolean))
  (return (`self.bNeedRest`)))

(fn `GetSpeed`
  (returns (Speed :type "Float (double-precision)"))
  (return (`KismetMathLibrary.VSizeXY` (`Actor.GetVelocity` (`self.GetOwner`)))))

(fn `InitializeRunSpeed`
  (params (RunSpeed :type "Float (double-precision)"))
  (set `self.RunSpeed` (`KismetMathLibrary.FMax` RunSpeed)))

(fn `RefreshStamina`
  (`self.IncreaseValue` (`self.RefreshStaminaValue`))
  (`self.SetNeedRest`))

(fn `SetNeedRest`
  (bind _returnvalue (< (`self.GetValue`) (`self.ValueToRest`)))
  (if (and _returnvalue (not (`self.bNeedRest`)))
    (`self.OnStartRest`))
  (set `self.bNeedRest` _returnvalue))

(fn `ShowDebug`
  (bind _wastetimerhandle (`self.WasteTimerHandle`))
  (`parent.ShowDebug`)
  (`KismetSystemLibrary.PrintString` (`KismetTextLibrary.Conv_TextToString` (`|FormatText` "Need Rest : {NR} \nRefreshTimer : {RT} \nWasteTimer : {WT} \nPauseWasteTimer : {PWT}" (`self.bNeedRest`) (`KismetSystemLibrary.K2_IsTimerActiveHandle` (`self.RefreshTimerHandle`)) (`KismetSystemLibrary.K2_IsTimerActiveHandle` _wastetimerhandle) (`KismetSystemLibrary.K2_IsTimerPausedHandle` _wastetimerhandle))) true true (struct :`R` 0.021219 :`G` 1.0 :`A` 1.0) 0.0))

(fn `StartRefresh`
  (if (and (< (`self.GetValue`) (`self.MaxFloatValue`)) (not (`KismetSystemLibrary.K2_IsTimerActiveHandle` (`self.RefreshTimerHandle`))))
    (`self.SetNeedRest`)
    (if (or (`self.GetValueEqualZero`) (`self.bNeedRest`))
      (`KismetSystemLibrary.K2_ClearAndInvalidateTimerHandle` (`self.WasteTimerHandle`)))
    (bind _returnvalue (`KismetSystemLibrary.K2_SetTimerDelegate` (`|CreateDelegate` :!event `RefreshStamina`) (`self.RefreshStaminaPeriod`) true (`self.TimeToStartRefresh`)))
    (set `self.RefreshTimerHandle` _returnvalue)))

(fn `StartRun`
  (if (`self.GetCanRun`)
    (`self.StopRefresh`)
    (if (`KismetSystemLibrary.K2_IsTimerPausedHandle` (`self.WasteTimerHandle`))
      (`KismetSystemLibrary.K2_UnPauseTimerHandle` (`self.WasteTimerHandle`))
      (else
        (bind _returnvalue (`KismetSystemLibrary.K2_SetTimerDelegate` (`|CreateDelegate` :!event `WasteStamina`) (`self.DecreaseStaminaPeriod`) true))
        (set `self.WasteTimerHandle` _returnvalue)))))

(fn `StopRefresh`
  (`KismetSystemLibrary.K2_ClearAndInvalidateTimerHandle` (`self.RefreshTimerHandle`)))

(fn `StopRun`
  (`KismetSystemLibrary.K2_PauseTimerHandle` (`self.WasteTimerHandle`))
  (`self.StartRefresh`))

(fn `WasteStamina`
  (bind _charactermovement (`self.GetCharacterMovement`))
  (`self.DecreaseValue` (`KismetMathLibrary.SelectFloat` 0.0 (`KismetMathLibrary.SelectFloat` (`self.DecreaseStaminaValue`) 0.0 (> (`self.GetSpeed`) (`self.RunSpeed`))) (`NavMovementComponent.IsFalling` _charactermovement))))