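; BP_FakeDoor is an interactable quest door that stages a short camera cutscene when used.
; Hits on its Box allow interaction, toggling a tooltip widget and custom-depth outline until used.
; StartInteract disables input, walks and turns the player to CharacterPosition, blends the view to the door and starts a timer.
; Helper functions play an opening montage with a follow-up timer and restore camera and input; timer targets are unclear.
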(event `self.ReceiveBeginPlay`
  (`Widget.SetVisibility` (`WidgetComponent.GetWidget` (`self.BP_WidgetComp`)) "Collapsed"))

(event `/Game/Immersion_game/Blueprints/Interfaces/BPI_Interact.CancelCanInteract`
  (`self.ActivateOutlinerAndTooltip` false))

(fn `ActivateOutlinerAndTooltip`
  (params (Active :type Boolean))
  (bind _returnvalue (or (not (`self.UseNow`)) Active))
  (`Widget.SetVisibility` (`WidgetComponent.GetWidget` (`self.BP_WidgetComp`)) (select `bool` _returnvalue :`false` "Collapsed" :`true` "Visible" :!type "ESlateVisibility Enum"))
  (`PrimitiveComponent.SetRenderCustomDepth` (`self.StaticMesh`) _returnvalue))

(fn `CanInteract`
  (params (Hit :type "HitResult Structure"))
  (returns (True :type Boolean))
  (if (== (`.HitComponent` (`GameplayStatics.BreakHitResult` Hit)) (`self.Box`))
    (if (not (`self.UseNow`))
      (`self.ActivateOutlinerAndTooltip` true))
    (return true)
    (else
      (return false))))

(fn `EndCutscene`
  (`PlayerController.SetViewTargetWithBlend` (`GameplayStatics.GetPlayerController` 0) (`GameplayStatics.GetPlayerCharacter` 0) 1.0 "VTBlend_Linear" 1.0 false)
  (`self.EnableInput` (`GameplayStatics.GetPlayerCharacter` 0) (`GameplayStatics.GetPlayerController` 0)))

(fn `Move and Rotate Character`
  (bind _returnvalue (`GameplayStatics.GetPlayerController` 0))
  (bind _characterposition (`self.CharacterPosition`))
  (`AIBlueprintHelperLibrary.SimpleMoveToLocation` _returnvalue (`SceneComponent.K2_GetComponentLocation` _characterposition))
  (`Controller.SetControlRotation` _returnvalue (`SceneComponent.K2_GetComponentRotation` _characterposition)))

(fn `NewFunction`
  (bind _montagelengtgh (`/Game/Immersion_game/Core/Character/BP_Character.PlayMontage` (cast `/Game/Immersion_game/Core/Character/BP_Character` (`GameplayStatics.GetPlayerCharacter` 0) :!pure true) "/Game/Resources/Animations/Hero/Opening_Montage.Opening_Montage" 1.0 false))
  (`KismetSystemLibrary.K2_SetTimerDelegate` (`|CreateDelegate` :!event `EndCutscene`) 0.01 false _montagelengtgh))

(fn `StartInteract`
  (params (InteractByActor :type "Actor Object Reference"))
  (returns (bSuccess :type Boolean) (ShouldPlayAnim :type Boolean))
  (`self.DisableInput` (`GameplayStatics.GetPlayerCharacter` 0) (`GameplayStatics.GetPlayerController` 0))
  (`self.Move and Rotate Character`)
  (`PlayerController.SetViewTargetWithBlend` (`GameplayStatics.GetPlayerController` 0) self 1.0 "VTBlend_Linear" 1.0 false)
  (`KismetSystemLibrary.K2_SetTimerDelegate` (`|CreateDelegate` :!event `NewFunction`) 0.01 false 0.5)
  (set `self.UseNow` true)
  (`self.ActivateOutlinerAndTooltip` false)
  (return true false))

(fn `UserConstructionScript`)