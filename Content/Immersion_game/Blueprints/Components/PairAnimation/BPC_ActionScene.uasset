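; Actor component that plays paired action scenes, aligning two characters while both play synchronized montages, with optional camera shake.
; Temporary TargetPoints serve as proxies to precompute final positions and facing in configurable order, optionally capsule-tracing to push the scene away from walls.
; A Timeline lerps location, actor rotation and control rotation while capsule Pawn collision is ignored, then restores collision and destroys the proxies.
; Start dispatchers fire and montage-length timers are set.
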(event `self.ReceiveBeginPlay`
  ;[1 1 1] Timeline не работает без тика
  (`self.SetComponentTickEnabled` true))

(event `self.TimelineStop`
  (`self.DebugFunction`)
  (`self.ToggleCharactersCollision` true)
  (`self.ClearInfoAfterScene`))

(event `self.TimelineProgress`
  (params (Value :type "Float (single-precision)"))
  (`self.Set Character Location` (`self.FirstCharacterLocation`) Value)
  (`self.Set Character Location` (`self.SecondCharacterLocation`) Value)
  (`self.Set Character Rotation` (`self.FirstCharacterRotation`) Value)
  (`self.Set Character Rotation` (`self.SecondCharacterRotation`) Value))

(fn `ClearInfoAfterScene`
  (set `self.First Character` null)
  (set `self.Second Character` null)
  (set `self.FirstCharacterRotation` (struct))
  (set `self.SecondCharacterRotation` (struct))
  (set `self.FirstCharacterLocation` (struct))
  (`Actor.K2_DestroyActor` (`self.FirstCharacterPlace`))
  (`Actor.K2_DestroyActor` (`self.SecondCharacterPlace`)))

(fn `CreateCharactersPlaces`
  (params (FirstChar :type "Character Object Reference") (SecondChar :type "Character Object Reference"))
  (`self.FirstCharacterPlace`
    (:`then`
      _)
    (:`else`
      (bind _returnvalue (`|SpawnActorFromClass` "/Script/Engine.TargetPoint" (`Actor.GetTransform` (`local.FirstChar`)) "Undefined" "OverrideRootScale" null null))
      (set `self.FirstCharacterPlace` _returnvalue)))
  (`self.SecondCharacterPlace`
    (:`then`)
    (:`else`
      (bind _returnvalue_2 (`|SpawnActorFromClass` "/Script/Engine.TargetPoint" (`Actor.GetTransform` (`local.SecondChar`)) "Undefined" "OverrideRootScale" null null))
      (set `self.SecondCharacterPlace` _returnvalue_2))))

(fn `DebugFunction`
  (bind _secondcharacterplace (`self.SecondCharacterPlace`))
  (if (`self.bShowDebug`)
    (`KismetSystemLibrary.PrintString` (`KismetTextLibrary.Conv_TextToString` (`|FormatText` "FLP : {FLP} \nSLP : {SLP}" (`KismetStringLibrary.Conv_VectorToString` (`KismetMathLibrary.InverseTransformLocation` (`Actor.GetTransform` _secondcharacterplace) (`Actor.K2_GetActorLocation` (`self.FirstCharacterPlace`)))) (`KismetStringLibrary.Conv_VectorToString` (`Actor.K2_GetActorLocation` _secondcharacterplace)))) true true (struct :`R` 1.0 :`B` 0.0409 :`A` 1.0) 15.0)
    (`KismetSystemLibrary.DrawDebugSphere` (`Actor.K2_GetActorLocation` (`self.FirstCharacterPlace`)) 25.0 12 (struct :`R` 0.008417 :`G` 1.0 :`A` 1.0) 15.0)
    (`KismetSystemLibrary.DrawDebugSphere` (`Actor.K2_GetActorLocation` (`self.SecondCharacterPlace`)) 25.0 12 (struct :`R` 1.0 :`B` 0.092549 :`A` 1.0) 15.0)))

(fn `PairActionScene`
  (params (FirstCharacter :type "Character Object Reference") (SecondCharacter :type "Character Object Reference") (LActionSceneInfo :type "/Game/Immersion_game/Blueprints/Components/PairAnimation/S_ActionSceneInfoAdvanced Structure"))
  (returns (FirstAnimTime :type "Float (double-precision)") (SecondAnimTime :type "Float (double-precision)"))
  (bind _firstcharacter (`local.FirstCharacter`))
  (bind _firstcharacter_2 (`local.FirstCharacter`))
  (bind _secondcharacter (`local.SecondCharacter`))
  (bind _secondcharacter_2 (`local.SecondCharacter`))
  (bind _lactionsceneinfo (`local.LActionSceneInfo`))
  (bind _lactionsceneinfo_2 (`local.LActionSceneInfo`))
  (set `self.First Character` FirstCharacter)
  (set `self.Second Character` SecondCharacter)
  (`self.CreateCharactersPlaces` FirstCharacter SecondCharacter)
  (switch `/Game/Immersion_game/Blueprints/Components/PairAnimation/E_ActionSceneRule` (`.ActionRule_42_DE64421D4AAF38229E5E21B842BA6528` (break `/Game/Immersion_game/Blueprints/Components/PairAnimation/S_ActionSceneInfoAdvanced` LActionSceneInfo))
    (:`NewEnumerator0`
      (`self.Save Character Location` _firstcharacter _secondcharacter_2 _lactionsceneinfo_2)
      (`self.Save Character Rotation` _firstcharacter_2 _secondcharacter _lactionsceneinfo_2))
    (:`NewEnumerator1`
      (`self.Save Character Rotation` _firstcharacter _secondcharacter_2 _lactionsceneinfo)
      (`self.Save Character Location` _firstcharacter_2 _secondcharacter _lactionsceneinfo)))
  ;[1 1 1] Animation
  (`self.OnStartFirstActionScene`)
  (`self.OnStartSecondActionScene`)
  (bind (_firstanimtime _secondanimtime) (`self.StartAnimation` (`local.FirstCharacter`) (`local.SecondCharacter`) (`local.LActionSceneInfo`)))
  (`KismetSystemLibrary.K2_SetTimerDelegate` (`|CreateDelegate` :!event `StopFirstActionScene`) _firstanimtime)
  (`KismetSystemLibrary.K2_SetTimerDelegate` (`|CreateDelegate` :!event `StopSecondActionScene`) _secondanimtime)
  (`self.PlayTimeline`)
  (`self.ToggleCharactersCollision` false)
  (return _firstanimtime _secondanimtime))

(fn `Rotate Character To`
  (params (FirstCharacterFromRotate :type "TargetPoint Object Reference") (SecondCharacterToRotate :type "TargetPoint Object Reference") (RotationInfo :type "/Game/Immersion_game/Blueprints/Components/PairAnimation/S_RotationInfo Structure (by ref)"))
  (locals (FirstToSecondControlRotation :type "Rotator Structure") (FirstToSecondLookRotation :type "Rotator Structure") (ActorStartRotation :type "Rotator Structure" :default (struct)) (ActorEndRotation :type "Rotator Structure" :default (struct)) (ActorStartControlRotation :type "Rotator Structure" :default (struct)) (ActorEndControlRotation :type "Rotator Structure" :default (struct)))
  (bind (_firsttosecondcontrolrotation_roll _firsttosecondcontrolrotation_pitch) (`KismetMathLibrary.BreakRotator` (`local.FirstToSecondControlRotation`)))
  (bind _firstcharacterfromrotate (`local.FirstCharacterFromRotate`))
  (bind (_returnvalue_roll _returnvalue_pitch) (`KismetMathLibrary.BreakRotator` (`Actor.K2_GetActorRotation` _firstcharacterfromrotate)))
  (set `local.FirstToSecondControlRotation` (`Actor.K2_GetActorRotation` (`local.FirstCharacterFromRotate`)))
  (set `local.FirstToSecondLookRotation` (`KismetMathLibrary.FindLookAtRotation` (`Actor.K2_GetActorLocation` FirstCharacterFromRotate) (`Actor.K2_GetActorLocation` SecondCharacterToRotate)))
  (set `local.ActorStartRotation` (`Actor.K2_GetActorRotation` _firstcharacterfromrotate))
  (bind _output_get (set `local.ActorEndRotation` (`KismetMathLibrary.MakeRotator` _returnvalue_roll _returnvalue_pitch (.yaw (`local.FirstToSecondLookRotation`)))))
  (`Actor.K2_SetActorRotation` (`local.FirstCharacterFromRotate`) _output_get false)
  (set `local.ActorStartControlRotation` (`Actor.K2_GetActorRotation` (`local.FirstCharacterFromRotate`)))
  (set `local.ActorEndControlRotation` (`KismetMathLibrary.MakeRotator` _firsttosecondcontrolrotation_roll _firsttosecondcontrolrotation_pitch (.yaw (`local.FirstToSecondLookRotation`))))
  (setmembers `/Game/Immersion_game/Blueprints/Components/PairAnimation/S_RotationInfo` :`StructRef` RotationInfo :`StartActorRotation` (`local.ActorStartRotation`) :`EndActorRotation` (`local.ActorEndRotation`) :`StartControlRotation` (`local.ActorStartControlRotation`) :`EndControlRotation` (`local.ActorEndControlRotation`)))

(fn `Save Character Location`
  (params (FirstCharacter :type "Character Object Reference") (SecondCharacter :type "Character Object Reference") (ActionScene :type "/Game/Immersion_game/Blueprints/Components/PairAnimation/S_ActionSceneInfoAdvanced Structure"))
  (locals (FirstToMove :type "TargetPoint Object Reference") (SecondToMove :type "TargetPoint Object Reference"))
  (bind ((`MoveCondition_25_175D3D824BE2EB7172882299507EDE9A` _movecondition)) (break `/Game/Immersion_game/Blueprints/Components/PairAnimation/S_ActionSceneInfoAdvanced` ActionScene))
  (bind _secondtomove (`local.SecondToMove`))
  (bind ((`ActionSceneLocation_33_65B498D74B2C80E750284B94EBD83449` _actionscenelocation) (`bCheckWall_47_CECA9E024E48067C80B955B22D950E0A` _bcheckwall)) (break `/Game/Immersion_game/Blueprints/Components/PairAnimation/S_ActionSceneInfoAdvanced` (`local.ActionScene`)))
  (bind (_returnvalue_x _returnvalue_y _returnvalue_z) (`KismetMathLibrary.BreakVector` (`Actor.K2_GetActorLocation` _secondtomove)))
  (bind (_x _y) (`KismetMathLibrary.BreakVector2D` _actionscenelocation))
  (bind _returnvalue (select `/Game/Immersion_game/Blueprints/Components/PairAnimation/E_MoveCondition` (`.MoveCondition_25_175D3D824BE2EB7172882299507EDE9A` (break `/Game/Immersion_game/Blueprints/Components/PairAnimation/S_ActionSceneInfoAdvanced` (`local.ActionScene`))) :`NewEnumerator0` (`local.SecondCharacter`) :`NewEnumerator1` (`local.FirstCharacter`)))
  (bind _returnvalue_2 (select `/Game/Immersion_game/Blueprints/Components/PairAnimation/E_MoveCondition` (`.MoveCondition_25_175D3D824BE2EB7172882299507EDE9A` (break `/Game/Immersion_game/Blueprints/Components/PairAnimation/S_ActionSceneInfoAdvanced` (`local.ActionScene`))) :`NewEnumerator0` (`local.FirstCharacter`) :`NewEnumerator1` (`local.SecondCharacter`)))
  (bind _returnvalue_3 (select `/Game/Immersion_game/Blueprints/Components/PairAnimation/E_MoveCondition` (`.MoveCondition_25_175D3D824BE2EB7172882299507EDE9A` (break `/Game/Immersion_game/Blueprints/Components/PairAnimation/S_ActionSceneInfoAdvanced` (`local.ActionScene`))) :`NewEnumerator0` (`local.FirstCharacter`) :`NewEnumerator1` (`local.SecondCharacter`)))
  (bind (_returnvalue_x_2 _returnvalue_y_2) (`KismetMathLibrary.BreakVector` (`KismetMathLibrary.TransformLocation` (`Actor.GetTransform` _secondtomove) (`KismetMathLibrary.MakeVector` _x _y))))
  (bind _capsulecomponent (`Character.CapsuleComponent` _returnvalue_3))
  (bind _returnvalue_4 (`CapsuleComponent.GetScaledCapsuleHalfHeight` _capsulecomponent))
  (bind _returnvalue_5 (+ (/ (`CapsuleComponent.GetScaledCapsuleHalfHeight` (`Character.CapsuleComponent` _returnvalue_3)) 4.0) (.z (`Actor.K2_GetActorLocation` _returnvalue_3))))
  ;[1 1 1] First
  (set `local.FirstToMove` (select `/Game/Immersion_game/Blueprints/Components/PairAnimation/E_MoveCondition` _movecondition :`NewEnumerator0` (`self.FirstCharacterPlace`) :`NewEnumerator1` (`self.SecondCharacterPlace`)))
  ;[1 1 1] Second
  (set `local.SecondToMove` (select `/Game/Immersion_game/Blueprints/Components/PairAnimation/E_MoveCondition` _movecondition :`NewEnumerator0` (`self.SecondCharacterPlace`) :`NewEnumerator1` (`self.FirstCharacterPlace`)))
  (if _bcheckwall
    (bind (_outhit _returnvalue_6) (`KismetSystemLibrary.CapsuleTraceSingleForObjects` (`KismetMathLibrary.MakeVector` (.x (`Actor.K2_GetActorLocation` (`local.SecondToMove`))) (.y (`Actor.K2_GetActorLocation` (`local.SecondToMove`))) _returnvalue_5) (`KismetMathLibrary.MakeVector` (.x (`KismetMathLibrary.MakeVector` _returnvalue_x_2 _returnvalue_y_2 _returnvalue_z)) (.y (`KismetMathLibrary.MakeVector` _returnvalue_x_2 _returnvalue_y_2 _returnvalue_z)) _returnvalue_5) (`KismetMathLibrary.FMax` (/ (`.SphereRadius` (`KismetSystemLibrary.GetComponentBounds` (`Character.Mesh` _returnvalue_3))) 4.0) (`CapsuleComponent.GetScaledCapsuleRadius` _capsulecomponent)) (- _returnvalue_4 (/ _returnvalue_4 4.0)) (`|MakeArray` "ObjectTypeQuery1" "ObjectTypeQuery2" :!type "EObjectTypeQuery Enum") false (`|MakeArray` (`self.First Character`) (`self.Second Character`) :!type "Actor Object Reference") (select `bool` (`self.bShowDebug`) :`true` "ForDuration" :!type "EDrawDebugTrace Enum")))
    (if _returnvalue_6
      (bind (_bblockinghit _binitialoverlap _time _distance _location _impactpoint _normal _impactnormal _physmat _hitactor _hitcomponent _hitbonename _bonename _hititem _elementindex _faceindex _tracestart _traceend) (`GameplayStatics.BreakHitResult` _outhit))
      (bind _returnvalue_7 (`KismetMathLibrary.GetForwardVector` (`KismetMathLibrary.FindLookAtRotation` _traceend _tracestart)))
      (`Actor.K2_SetActorLocation` (`local.SecondToMove`) (+ (`Actor.K2_GetActorLocation` (`local.SecondToMove`)) (+ (* _returnvalue_7 (`CapsuleComponent.GetScaledCapsuleRadius` (`Character.CapsuleComponent` (select `/Game/Immersion_game/Blueprints/Components/PairAnimation/E_MoveCondition` (`.MoveCondition_25_175D3D824BE2EB7172882299507EDE9A` (break `/Game/Immersion_game/Blueprints/Components/PairAnimation/S_ActionSceneInfoAdvanced` (`local.ActionScene`))) :`NewEnumerator0` (`local.FirstCharacter`) :`NewEnumerator1` (`local.SecondCharacter`))))) (* _returnvalue_7 (`KismetMathLibrary.Vector_Distance` _impactpoint _traceend)))) false false)))
  (`Actor.K2_SetActorLocation` (`local.FirstToMove`) (`KismetMathLibrary.MakeVector` _returnvalue_x_2 _returnvalue_y_2 _returnvalue_z) false false)
  (setmembers `/Game/Immersion_game/Blueprints/Components/PairAnimation/S_LocationInfo` :`StructRef` (`self.FirstCharacterLocation`) :`LocatingCharacter` _returnvalue_2 :`StartActorLocation` (`Actor.K2_GetActorLocation` _returnvalue_2) :`EndActorLocation` (`Actor.K2_GetActorLocation` (`local.FirstToMove`)))
  (setmembers `/Game/Immersion_game/Blueprints/Components/PairAnimation/S_LocationInfo` :`StructRef` (`self.SecondCharacterLocation`) :`LocatingCharacter` _returnvalue :`StartActorLocation` (`Actor.K2_GetActorLocation` _returnvalue) :`EndActorLocation` (`Actor.K2_GetActorLocation` (`local.SecondToMove`))))

(fn `Save Character Rotation`
  (params (FirstCharacterToRotate :type "Character Object Reference") (SecondCharacterToRotate :type "Character Object Reference") (LActionScene :type "/Game/Immersion_game/Blueprints/Components/PairAnimation/S_ActionSceneInfoAdvanced Structure"))
  (bind _secondcharacterplace (`self.SecondCharacterPlace`))
  (bind _firstcharacterplace (`self.FirstCharacterPlace`))
  (bind _secondcharacterplace_2 (`self.SecondCharacterPlace`))
  (bind _firstcharacterplace_2 (`self.FirstCharacterPlace`))
  (switch `/Game/Immersion_game/Blueprints/Components/PairAnimation/E_RotateCondition` (`.RotateCondition_27_49C2FC804A6E2ADDC3D810B8EF31AAA1` (break `/Game/Immersion_game/Blueprints/Components/PairAnimation/S_ActionSceneInfoAdvanced` LActionScene))
    (:`NewEnumerator0`
      (bind _structout (setmembers `/Game/Immersion_game/Blueprints/Components/PairAnimation/S_RotationInfo` :`StructRef` (`self.FirstCharacterRotation`) :`RotatingCharacter` (`local.FirstCharacterToRotate`)))
      (`self.Rotate Character To` _firstcharacterplace_2 _secondcharacterplace _structout))
    (:`NewEnumerator1`
      (bind _structout_2 (setmembers `/Game/Immersion_game/Blueprints/Components/PairAnimation/S_RotationInfo` :`StructRef` (`self.FirstCharacterRotation`) :`RotatingCharacter` (`local.SecondCharacterToRotate`)))
      (`self.Rotate Character To` _secondcharacterplace _firstcharacterplace_2 _structout_2))
    (:`NewEnumerator3`
      (bind _structout_3 (setmembers `/Game/Immersion_game/Blueprints/Components/PairAnimation/S_RotationInfo` :`StructRef` (`self.FirstCharacterRotation`) :`RotatingCharacter` (`local.FirstCharacterToRotate`)))
      (bind _structout_4 (setmembers `/Game/Immersion_game/Blueprints/Components/PairAnimation/S_RotationInfo` :`StructRef` (`self.SecondCharacterRotation`) :`RotatingCharacter` (`local.SecondCharacterToRotate`)))
      (`self.Rotate Character To` _firstcharacterplace _secondcharacterplace_2 _structout_3)
      (`self.Rotate Character To` _secondcharacterplace_2 _firstcharacterplace _structout_4))))

(fn `Set Character Location`
  (params (LocationInfo :type "/Game/Immersion_game/Blueprints/Components/PairAnimation/S_LocationInfo Structure") (Value :type "Float (double-precision)"))
  (bind (_locatingcharacter _startactorlocation _endactorlocation) (break `/Game/Immersion_game/Blueprints/Components/PairAnimation/S_LocationInfo` LocationInfo))
  (bind (_returnvalue_x _returnvalue_y) (`KismetMathLibrary.BreakVector` (`KismetMathLibrary.VLerp` _startactorlocation _endactorlocation Value)))
  (bind (_returnvalue_x_2 _returnvalue_y_2 _returnvalue_z) (`KismetMathLibrary.BreakVector` (`Actor.K2_GetActorLocation` _locatingcharacter)))
  (`/Engine/EditorBlueprintResources/StandardMacros.IsValid` _locatingcharacter
    (:`Is Valid`
      (`Actor.K2_SetActorLocation` _locatingcharacter (`KismetMathLibrary.MakeVector` _returnvalue_x _returnvalue_y _returnvalue_z) false false))))

(fn `Set Character Rotation`
  (params (RotationInfo :type "/Game/Immersion_game/Blueprints/Components/PairAnimation/S_RotationInfo Structure") (Value :type "Float (double-precision)"))
  (bind ((`RotatingCharacter_13_72ECA6E64F083C6CBEC0E0B37C2D27E5` _rotatingcharacter) (`StartActorRotation_5_20BAA1484FEE626A37074E8AB3741835` _startactorrotation) (`EndActorRotation_4_B5FF81364F5AF24534515EB04EAE67E4` _endactorrotation)) (break `/Game/Immersion_game/Blueprints/Components/PairAnimation/S_RotationInfo` RotationInfo))
  (bind ((`StartControlRotation_9_456824DD44528CBCC31779B8638DF4A4` _startcontrolrotation) (`EndControlRotation_10_A08105C64AEF6B69F69DC48108DEE02D` _endcontrolrotation)) (break `/Game/Immersion_game/Blueprints/Components/PairAnimation/S_RotationInfo` (`local.RotationInfo`)))
  (bind _returnvalue (`Pawn.GetController` _rotatingcharacter))
  (`/Engine/EditorBlueprintResources/StandardMacros.IsValid` _rotatingcharacter
    (:`Is Valid`
      (`Actor.K2_SetActorRotation` _rotatingcharacter (`KismetMathLibrary.RLerp` _startactorrotation _endactorrotation Value true) false)
      (`/Engine/EditorBlueprintResources/StandardMacros.IsValid` _returnvalue
        (:`Is Valid`
          (`Controller.SetControlRotation` _returnvalue (`KismetMathLibrary.RLerp` _startcontrolrotation _endcontrolrotation Value true)))))))

(fn `StartAnimation`
  (params (FirstCharacter :type "Character Object Reference") (SecondCharacter :type "Character Object Reference") (actionSceneInfo :type "/Game/Immersion_game/Blueprints/Components/PairAnimation/S_ActionSceneInfoAdvanced Structure"))
  (returns (FirstAnimTime :type "Float (single-precision)") (SecondAnimTime :type "Float (single-precision)"))
  (bind ((`FirstCharAM_45_329A5B204E96968AA650E8BB906CB21B` _firstcharam) (`SecondCharAM_44_C61DD1D649196182032954BDE57AF222` _secondcharam)) (break `/Game/Immersion_game/Blueprints/Components/PairAnimation/S_ActionSceneInfoAdvanced` actionSceneInfo))
  (bind _returnvalue (`Character.PlayAnimMontage` (`local.FirstCharacter`) _firstcharam 1.0 "None"))
  (bind _returnvalue_2 (`Character.PlayAnimMontage` (`local.SecondCharacter`) _secondcharam 1.0 "None"))
  (if (`Pawn.IsPlayerControlled` (`local.FirstCharacter`))
    (`PlayerCameraManager.StartCameraShake` :`self` (`GameplayStatics.GetPlayerCameraManager` 0) :`ShakeClass` (`.ActionSceneCamera_32_41598A4D49D1A5709656D386D9B4B811` (break `/Game/Immersion_game/Blueprints/Components/PairAnimation/S_ActionSceneInfoAdvanced` (`local.actionSceneInfo`)))))
  (return (`KismetMathLibrary.FMax` _returnvalue 0.001) (`KismetMathLibrary.FMax` _returnvalue_2 0.001)))

(fn `StopFirstActionScene`
  (`self.OnStopFirstActionScene`))

(fn `StopSecondActionScene`
  (`self.OnStopSecondActionScene`))

(fn `ToggleCharactersCollision`
  (params (bToggle :type Boolean))
  (locals (LocalFirstResponse :type "ECollisionResponse Enum") (LocalSecondResponse :type "ECollisionResponse Enum"))
  (set `local.LocalFirstResponse` (select `bool` (`local.bToggle`) :`false` "ECR_Ignore" :`true` (`self.FirstCharacterResponse`)))
  (set `local.LocalSecondResponse` (select `bool` (`local.bToggle`) :`false` "ECR_Ignore" :`true` (`self.SecondCharacterResponse`)))
  (set `self.FirstCharacterResponse` (select `bool` (`local.bToggle`) :`false` (`PrimitiveComponent.GetCollisionResponseToChannel` (`Character.CapsuleComponent` (`self.First Character`)) "ECC_Pawn") :`true` "ECR_Ignore"))
  (set `self.SecondCharacterResponse` (select `bool` (`local.bToggle`) :`false` (`PrimitiveComponent.GetCollisionResponseToChannel` (`Character.CapsuleComponent` (`self.Second Character`)) "ECC_Pawn") :`true` "ECR_Ignore"))
  (`PrimitiveComponent.SetCollisionResponseToChannel` (`Character.CapsuleComponent` (`self.First Character`)) "ECC_Pawn" (`local.LocalFirstResponse`))
  (`PrimitiveComponent.SetCollisionResponseToChannel` (`Character.CapsuleComponent` (`self.Second Character`)) "ECC_Pawn" (`local.LocalSecondResponse`)))