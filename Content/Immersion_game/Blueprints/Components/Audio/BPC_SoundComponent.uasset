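; BPC_SoundComponent is an actor component that gives its owner a single managed audio source for playing sounds.
; InitializeAudioComponent adds an AudioComponent to the owner, attaches it to a given component and socket, and applies the stored attenuation settings.
; PlayAudio validates the component and sound, then swaps and plays the sound, either interrupting current playback when PlayNew is set or only when nothing is playing.
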(fn `GetAudioComponent`
  (returns (AudioComponent :type "AudioComponent Object Reference"))
  (return (`self.AudioComponent`)))

(fn `InitializeAudioComponent`
  (params (ComponentToAttach :type "SceneComponent Object Reference") (SocketToAttach :type Name))
  (bind _returnvalue (`|AddComponentByClass` :`self` (`self.GetOwner`) :`Class` "/Script/Engine.AudioComponent"))
  (bind _output_get (set `self.AudioComponent` _returnvalue))
  (`SceneComponent.K2_AttachToComponent` _output_get (`local.ComponentToAttach`) (`local.SocketToAttach`) "KeepRelative" "KeepRelative" "KeepRelative" true)
  (set `AudioComponent.AttenuationSettings` (`self.Attenuation Settings`) _output_get))

(fn `PlayAudio`
  (params (SoundToPlay :type "SoundBase Object Reference") (bPlayNew :type Boolean))
  (bind _audiocomponent (`self.AudioComponent`))
  (`self.AudioComponent`
    (:`then`
      (`/Engine/EditorBlueprintResources/StandardMacros.IsValid` (`local.SoundToPlay`)
        (:`Is Valid`
          (if bPlayNew
            (`AudioComponent.SetSound` _audiocomponent (`local.SoundToPlay`) :!label _label)
            (`AudioComponent.Play` _audiocomponent 0.0)
            (elif (not (`AudioComponent.IsPlaying` (`self.AudioComponent`)))
              (goto _label))))))
    (:`else`)))