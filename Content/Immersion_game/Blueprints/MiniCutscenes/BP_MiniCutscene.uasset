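; Mini-cutscene actor that briefly pulls the player's view onto itself, with blend times and curves set by variables.
; TriggerScript, shaped as an overlap handler, disables player input and blends the view target to this actor.
; It then starts a timer delayed by SeeObjectTime, presumably to call SetViewTargetToCharacter, which restores input and blends back to the character.
; No overlap binding is shown, and the event graph is empty.
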(fn `SetViewTargetToCharacter`
  (bind _returnvalue (`GameplayStatics.GetPlayerController` 0))
  (bind _returnvalue_2 (`GameplayStatics.GetPlayerCharacter` 0))
  (`self.EnableInput` _returnvalue_2 _returnvalue)
  (`PlayerController.SetViewTargetWithBlend` _returnvalue _returnvalue_2 (`self.ObjectToCharactertBlendTime`) (`self.ObjectToCharacterttBlendFunc`) (`self.ObjectToCharacterttBlendExp`) true))

(fn `SetViewTargetToObject`
  (bind _returnvalue (`GameplayStatics.GetPlayerController` 0))
  (`self.DisableInput` (`GameplayStatics.GetPlayerCharacter` 0) _returnvalue)
  (`PlayerController.SetViewTargetWithBlend` _returnvalue self (`self.CharacterToObjectBlendTime`) (`self.CharacterToObjectBlendFunc`) (`self.CharacterToObjectBlendExp`) true))

(fn `TriggerScript`
  (params (OverlappedComponent :type "PrimitiveComponent Object Reference") (OtherActor :type "Actor Object Reference") (OtherComp :type "PrimitiveComponent Object Reference") (OtherBodyIndex :type Integer) (bFromSweep :type Boolean) (SweepResult :type "HitResult Structure (by ref)"))
  (`self.SetViewTargetToObject`)
  (`KismetSystemLibrary.K2_SetTimerDelegate` (`|CreateDelegate` :!event `SetViewTargetToCharacter`) 0.01 false (`self.SeeObjectTime`))
  (return))

(fn `UserConstructionScript`)