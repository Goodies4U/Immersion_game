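; Interaction component that finds usable objects in front of the player camera and starts or stops interacting with them.
; A looping timer drives camera sphere traces, tracking the current BPI_Interact target and sending can-interact and cancel messages.
; StartInteract messages that target and optionally plays a pickup montage, chosen by object height against the pelvis and sped up with movement speed.
; Character rotation toward the target exists but is disconnected.
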(event `self.ReceiveBeginPlay`
  (`KismetSystemLibrary.K2_SetTimerDelegate` (`|CreateDelegate` :!event `Checking`) 0.05 true))

(event `StopInteract`
  (bind _able_to_interact_with_this_actor (`self.Able to interact with this actor`)
    (:`then`
      (message `/Game/Immersion_game/Blueprints/Interfaces/BPI_Interact.StopInteract` _able_to_interact_with_this_actor))
    (:`else`)))

(fn `Checking`
  (locals (LocalHit :type "HitResult Structure"))
  (bind _localhit (`local.LocalHit`))
  (bind (_bblockinghit _binitialoverlap _time _distance _location _impactpoint _normal _impactnormal _physmat _hitactor) (`GameplayStatics.BreakHitResult` (`local.LocalHit`)))
  (if (not (`self.bStopTraceCheck`))
    (`|ExecutionSequence`
      (:`then_0`
        (bind (_outhits _returnvalue) (`self.TraceFromActiveCamera`))
        (if _returnvalue
          (for _array_element _outhits
            (set `local.LocalHit` _array_element)
            (`self.Able to interact with this actor`
              (:`then`
                (if (not (== (`self.Able to interact with this actor`) (`.HitActor` (`GameplayStatics.BreakHitResult` (`local.LocalHit`)))))
                  (message `/Game/Immersion_game/Blueprints/Interfaces/BPI_Interact.CancelCanInteract` (`self.Able to interact with this actor`))
                  (if (`KismetSystemLibrary.DoesImplementInterface` (`.HitActor` (`GameplayStatics.BreakHitResult` (`local.LocalHit`))) "/Game/Immersion_game/Blueprints/Interfaces/BPI_Interact.BPI_Interact_C") :!label _label
                    (bind _true (message `/Game/Immersion_game/Blueprints/Interfaces/BPI_Interact.CanInteract` (`.HitActor` (`GameplayStatics.BreakHitResult` _localhit)) _localhit (`self.GetOwner`)))
                    (if _true
                      (set `self.Able to interact with this actor` (select `bool` _true :`true` _hitactor))
                      (else
                        (message `/Game/Immersion_game/Blueprints/Interfaces/BPI_Interact.CancelCanInteract` _hitactor)
                        (set `self.Able to interact with this actor` null)))
                    (else
                      (set `self.Able to interact with this actor` null)))))
              (:`else`
                (goto _label))))
          (else
            (bind _able_to_interact_with_this_actor (`self.Able to interact with this actor`)
              (:`then`
                (message `/Game/Immersion_game/Blueprints/Interfaces/BPI_Interact.CancelCanInteract` _able_to_interact_with_this_actor)
                (set `self.Able to interact with this actor` null))
              (:`else`)))))
      (:`then_1`
        (goto _label_2 :!via `Reset`)))
    (else
      (`/Engine/EditorBlueprintResources/StandardMacros.DoOnce` false :!label _label_2
        (:`Completed`
          (message `/Game/Immersion_game/Blueprints/Interfaces/BPI_Interact.CancelCanInteract` (`self.Able to interact with this actor`))
          (set `self.Able to interact with this actor` null))))))

(fn `RotateCharacterToTarget`
  (bind (_targetrotation_roll _targetrotation_pitch _targetrotation_yaw) (`KismetMathLibrary.BreakRotator` (`self.TargetRotation`)))
  (bind _targetrotation (`self.TargetRotation`))
  (bind (_returnvalue_roll _returnvalue_pitch _returnvalue_yaw) (`KismetMathLibrary.BreakRotator` (`Controller.GetControlRotation` (`GameplayStatics.GetPlayerController` 0))))
  (bind (_returnvalue_roll_2 _returnvalue_pitch_2 _returnvalue_yaw_2) (`KismetMathLibrary.BreakRotator` (`Controller.GetControlRotation` (`GameplayStatics.GetPlayerController` 0))))
  (if (== _returnvalue_yaw_2 _targetrotation_yaw)
    (`KismetSystemLibrary.K2_ClearAndInvalidateTimerHandle` (`self.RotateTimer`))
    (else
      (`Controller.SetControlRotation` (`GameplayStatics.GetPlayerController` 0) (`KismetMathLibrary.RInterpTo` (`Actor.K2_GetActorRotation` (`GameplayStatics.GetPlayerCharacter` 0)) _targetrotation (`GameplayStatics.GetWorldDeltaSeconds`) 2.0))
      (`Actor.K2_SetActorRotation` (`GameplayStatics.GetPlayerCharacter` 0) (`KismetMathLibrary.MakeRotator` 0.0 0.0 (`KismetMathLibrary.FInterpTo` _returnvalue_yaw (.yaw _targetrotation) (`GameplayStatics.GetWorldDeltaSeconds`) 2.0)) false))))

(fn `StartInteract`
  (returns (bSuccess :type Boolean))
  (bind (_returnvalue_x _returnvalue_y _returnvalue_z) (`KismetMathLibrary.BreakVector` (`Actor.K2_GetActorLocation` (`self.Able to interact with this actor`))))
  (bind _asbp_character (cast `/Game/Immersion_game/Core/Character/BP_Character` (`GameplayStatics.GetPlayerCharacter` 0) :!pure true))
  (bind (_returnvalue_x_2 _returnvalue_y_2 _returnvalue_z_2) (`KismetMathLibrary.BreakVector` (`SceneComponent.GetSocketLocation` (`Character.Mesh` (`GameplayStatics.GetPlayerCharacter` 0)) "Pelvis")))
  (`self.Able to interact with this actor`
    (:`then`
      (bind (_bsuccess _bshouldplayanim _bshouldrotatecharactertoobject) (message `/Game/Immersion_game/Blueprints/Interfaces/BPI_Interact.StartInteract` (`self.Able to interact with this actor`) (`self.GetOwner`)))
      (`|ExecutionSequence`
        (:`then_0`
          (if _bshouldplayanim
            (`/Game/Immersion_game/Core/Character/BP_Character.PlayMontage` _asbp_character (select `bool` (< _returnvalue_z _returnvalue_z_2) :`false` "/Game/Resources/Animations/Hero/AM_PickUp_02.AM_PickUp_02" :`true` "/Game/Resources/Animations/Hero/AM_PickUp_01.AM_PickUp_01" :!type "AnimMontage Object Reference") (`KismetMathLibrary.MapRangeClamped` (`KismetMathLibrary.VSize` (`MovementComponent.Velocity` (`Character.CharacterMovement` _asbp_character))) 100.0 650.0 2.0 4.0) false)))
        (:`then_1`
          (if _bshouldrotatecharactertoobject
            _))
        (:`then_2`
          (return _bsuccess))))
    (:`else`)))

(fn `StopRotateToTarget`
  (`KismetSystemLibrary.K2_ClearAndInvalidateTimerHandle` (`self.RotateTimer`)))

(fn `ToggleChecking`
  (params (bToggleChecking :type Boolean))
  (bind _output_get (set `self.bStopTraceCheck` (not bToggleChecking)))
  (if (not _output_get)
    (bind _able_to_interact_with_this_actor (`self.Able to interact with this actor`)
      (:`then`
        (message `/Game/Immersion_game/Blueprints/Interfaces/BPI_Interact.CancelCanInteract` _able_to_interact_with_this_actor)
        (set `self.Able to interact with this actor` null))
      (:`else`))))

(fn `TraceFromActiveCamera`
  (returns (OutHits :type "Array of HitResult Structure") (ReturnValue :type Boolean))
  (bind _playercameramanager (`PlayerController.PlayerCameraManager` (`GameplayStatics.GetPlayerController` 0)))
  (bind _returnvalue (`Actor.K2_GetActorLocation` _playercameramanager))
  (bind _returnvalue_2 (`Actor.GetActorForwardVector` _playercameramanager))
  (bind (_outhits _returnvalue_3) (`KismetSystemLibrary.SphereTraceMulti` (+ _returnvalue _returnvalue_2) (+ _returnvalue (* _returnvalue_2 (`self.MaxIntreractionDistance`))) (`self.MaxInteractRadius`) "TraceTypeQuery1" false (`|MakeArray` (`self.GetOwner`)) (select `bool` (`self.bDebug`) :`true` "ForDuration" :!type "EDrawDebugTrace Enum") true (struct :`R` 1.0 :`A` 1.0) (struct :`G` 1.0 :`A` 1.0) 0.0))
  (return _outhits _returnvalue_3))