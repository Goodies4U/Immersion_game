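; BP_ParentTool is a base Blueprint for tools with primary and secondary actions.
; Start and stop events for each action forward to matching logic functions, and BeginPlay calls Initialization; these functions are empty stubs, apparently for child tools to override.
; Destroyed stops both actions, and a getter and setter expose the IsUseItem state.
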(event `self.ReceiveBeginPlay`
  (`self.Initialization`))

(event `self.StartPrimaryAction`
  (`self.StartPrimaryActionLogic`))

(event `self.StopPrimaryAction`
  (`self.StopPrimaryActionLogic`))

(event `self.StartSecondaryAction`
  (`self.StartSecondaryActionLogic`))

(event `self.StopSecondaryAction`
  (`self.StopSecondaryActionLogic`))

(event `self.ReceiveDestroyed`
  (`self.StopPrimaryAction`)
  (`self.StopSecondaryAction`))

(fn `GetIsUse`
  (returns (bIsUseItem :type Boolean))
  (return (`self.bIsUseItem`)))

(fn `Initialization`)

(fn `SetIsUse`
  (params (bIsUseItem :type Boolean))
  (set `self.bIsUseItem` bIsUseItem))

(fn `StartPrimaryActionLogic`)

(fn `StartSecondaryActionLogic`)

(fn `StopPrimaryActionLogic`)

(fn `StopSecondaryActionLogic`)

(fn `UserConstructionScript`)