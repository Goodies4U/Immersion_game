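; Interactable shadow puzzle where the player rotates a model to match a target orientation.
; Interacting consumes NeededItem from BPC_MiniInventory and loads its data table mesh, which previews at construction and is cleared on BeginPlay.
; BeginPlay saves RotatePoint's placed rotation as the solution, then zeroes it.
; Look input rotates the pivot with a debug print when close; Select within a looser tolerance marks success and timeline-lerps the model to the solution.
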(event `self.ReceiveBeginPlay`
  (bind _rotatepoint (`self.RotatePoint`))
  (`parent.ReceiveBeginPlay`)
  (`StaticMeshComponent.SetStaticMesh` (`self.ShadowModel`) null)
  (set `self.ShadowRotation` (`SceneComponent.K2_GetComponentRotation` _rotatepoint))
  (`SceneComponent.K2_SetWorldRotation` :`self` _rotatepoint))

(event `EnhancedInput|/Game/DEV/ThirdPerson/Input/Actions/IA_Look`
  (params (ActionValue :type "Vector2D Structure") (ElapsedSeconds :type "Float (double-precision)") (TriggeredSeconds :type "Float (double-precision)") (InputAction :type "InputAction Object Reference" :default "/Game/DEV/ThirdPerson/Input/Actions/IA_Look.IA_Look"))
  (bind _rotatepoint (`self.RotatePoint`))
  (:`Triggered`
    (if (not (`self.bSuccess`))
      (`SceneComponent.K2_SetWorldRotation` _rotatepoint (`KismetMathLibrary.ComposeRotators` (`KismetMathLibrary.MakeRotator` ActionValue_X 0.0 ActionValue_Y) (`SceneComponent.K2_GetComponentRotation` _rotatepoint)) false false)
      (if (== (`SceneComponent.K2_GetComponentRotation` (`self.RotatePoint`)) (`self.ShadowRotation`) :`ErrorTolerance` 10.0)
        (`KismetSystemLibrary.PrintString` "Good" true true (struct :`R` 1.0 :`B` 0.056662 :`A` 1.0) 0.0)))))

(event `EnhancedInput|/Game/Immersion_game/Inputs/Actions/IA_SelectItem`
  (params (ActionValue :type Boolean) (ElapsedSeconds :type "Float (double-precision)") (TriggeredSeconds :type "Float (double-precision)") (InputAction :type "InputAction Object Reference" :default "/Game/Immersion_game/Inputs/Actions/IA_SelectItem.IA_SelectItem"))
  (:`Started`
    (if (not (`self.bSuccess`))
      (if (== (`SceneComponent.K2_GetComponentRotation` (`self.RotatePoint`)) (`self.ShadowRotation`) :`ErrorTolerance` 20.0)
        (set `self.bSuccess` true)
        (set `self.SuccessRotation` (`SceneComponent.K2_GetComponentRotation` (`self.ShadowModel`)))
        (bind (_direction _successalpha) (`Timeline|ModelToSuccess` :!via `PlayFromStart`)
          (:`Update`
            (`SceneComponent.K2_SetWorldRotation` (`self.ShadowModel`) (`KismetMathLibrary.RLerp` (`self.SuccessRotation`) (`self.ShadowRotation`) _successalpha true) false false)))))))

(fn `CanInteract`
  (params (Hit :type "HitResult Structure") (QueryFromActor :type "Actor Object Reference"))
  (returns (True :type Boolean))
  (if (`self.bIsHaveModel`)
    (bind _true (`parent.CanInteract` Hit QueryFromActor))
    (return _true)
    (else
      (`self.ToggleInteractFX` true)
      (return true))))

(fn `StartInteract`
  (params (InteractByActor :type "Actor Object Reference"))
  (returns (bSuccess :type Boolean) (bShouldPlayAnim :type Boolean) (bShouldRotateCharacterToObject :type Boolean))
  (if (and (not (`self.bIsHaveModel`)) (not (`KismetSystemLibrary.IsValid` (`StaticMeshComponent.StaticMesh` (`self.ShadowModel`)))))
    (bind _bsuccess (`/Game/Immersion_game/Blueprints/Components/MiniInventrory/BPC_MiniInventory.TryUseItem` (`self.GetComponentByClass` InteractByActor "/Game/Immersion_game/Blueprints/Components/MiniInventrory/BPC_MiniInventory.BPC_MiniInventory_C") (`self.NeededItem`)))
    (if _bsuccess
      (bind _out_row (`self.GetDataTableRow`)
        (:`then`
          (`StaticMeshComponent.SetStaticMesh` (`self.ShadowModel`) (`.Model` (break `ItemInfo` _out_row)))
          (set `self.bIsHaveModel` true)
          (bind _bsuccess_2 (`parent.StartInteract` (`local.InteractByActor`)))
          (return _bsuccess_2 false false)))
      (else
        (return false false false)))
    (else
      (bind _bsuccess_3 (`parent.StartInteract` (`local.InteractByActor`)))
      (return _bsuccess_3 false false))))

(fn `UserConstructionScript`
  (bind _shadowmodel (`self.ShadowModel`))
  (`parent.UserConstructionScript`)
  (bind _out_row (`self.GetDataTableRow`)
    (:`then`
      (`StaticMeshComponent.SetStaticMesh` _shadowmodel (`.Model` (break `ItemInfo` _out_row))))
    (:`fail`
      (`StaticMeshComponent.SetStaticMesh` _shadowmodel null))))