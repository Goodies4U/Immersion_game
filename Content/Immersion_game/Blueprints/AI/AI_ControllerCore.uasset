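; AI_ControllerCore is an AI controller that starts the behavior tree assigned to the pawn it possesses.
; On possess it reads the run info from the pawn's BPC_BehaviorTreeComponent and, if that succeeds, runs the behavior tree it supplies.
; It then sets the StatueState blackboard key to a fixed initial enum value.
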(event `self.ReceivePossess`
  (params (PossessedPawn :type "Pawn Object Reference"))
  (bind _returnvalue (`self.GetComponentByClass` PossessedPawn "/Game/Immersion_game/Blueprints/AI/BPC_BehaviorTreeComponent.BPC_BehaviorTreeComponent_C"))
  (bind (_bsuccess _s_ai_info) (`/Game/Immersion_game/Blueprints/AI/BPC_BehaviorTreeComponent.GetRunAIInfo` _returnvalue))
  (`/Engine/EditorBlueprintResources/StandardMacros.IsValid` PossessedPawn
    (:`Is Valid`
      (`/Engine/EditorBlueprintResources/StandardMacros.IsValid` _returnvalue
        (:`Is Valid`
          (if _bsuccess
            (`self.RunBehaviorTree` (`.BehaviorTree_2_FAAE71E9455CF6EDF0B05B93EB9652C1` (break `/Game/Immersion_game/Blueprints/AI/S_AI_Info` _s_ai_info)))
            ;[1 0 0] !!!
            (`BlackboardComponent.SetValueAsEnum` (`AIBlueprintHelperLibrary.GetBlackboard` null) "StatueState" (enumliteral `/Game/Immersion_game/Blueprints/AI/Statue/E_StatueState` "NewEnumerator1"))))))))

(fn `UserConstructionScript`)