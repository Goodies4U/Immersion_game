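; Game mode that coordinates saving and loading of named slots through BP_SaveGame objects.
; SaveGame loads the existing slot or creates a new save object, broadcasts OnSaveGame so listeners can access it, then writes it to the slot.
; LoadGame reads an existing slot and broadcasts OnLoadGame with the loaded object, doing nothing if the slot is missing.
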(fn `LoadGame`
  (params (SlotName :type String))
  (bind _returnvalue (`GameplayStatics.DoesSaveGameExist` SlotName))
  (if _returnvalue
    (bind _returnvalue_2 (`GameplayStatics.LoadGameFromSlot` (`local.SlotName`)))
    (bind _asbp_save_game (cast `/Game/Immersion_game/Blueprints/AutosavesGame/BP_SaveGame` _returnvalue_2))
    (`self.OnLoadGame` _asbp_save_game)))

(fn `SaveGame`
  (params (SlotName :type String))
  (locals (LocalSaveGame :type "/Game/Immersion_game/Blueprints/AutosavesGame/BP_SaveGame Object Reference"))
  (`|ExecutionSequence`
    (:`then_0`
      (bind _returnvalue (`GameplayStatics.DoesSaveGameExist` (`local.SlotName`)))
      (if _returnvalue
        (bind _returnvalue_2 (`GameplayStatics.LoadGameFromSlot` (`local.SlotName`)))
        (bind _asbp_save_game (cast `/Game/Immersion_game/Blueprints/AutosavesGame/BP_SaveGame` _returnvalue_2)
          (:`then`
            (set `local.LocalSaveGame` _asbp_save_game))
          (:`CastFailed`
            (return)))
        (else
          (bind _returnvalue_3 (`GameplayStatics.CreateSaveGameObject` "/Game/Immersion_game/Blueprints/AutosavesGame/BP_SaveGame.BP_SaveGame_C"))
          (set `local.LocalSaveGame` _returnvalue_3))))
    (:`then_1`
      (`self.OnSaveGame` (`local.LocalSaveGame`)))
    (:`then_2`
      (`GameplayStatics.SaveGameToSlot` (`local.LocalSaveGame`) (`local.SlotName`)))))

(fn `UserConstructionScript`)