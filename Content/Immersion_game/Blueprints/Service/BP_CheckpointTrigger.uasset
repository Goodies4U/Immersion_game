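; Checkpoint trigger that registers itself as the player's latest checkpoint in BP_GameMode.
; On BeginPlay it caches the starting transforms of its assigned statues and pickup objects in parallel arrays, indexed like the actor lists.
; TriggerScript stores the checkpoint reference and sets the has-checkpoint flag on the game mode, without filtering the overlapping actor.
; The respawn itself is not performed in this Blueprint.
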(event `self.ReceiveBeginPlay`
  (for (_array_element _array_index) (`self.StatuesToRespawn`)
    (`KismetArrayLibrary.Array_Set` (`self.StatuesTransorms`) _array_index (`self.GetTransform` _array_element) true))
  (for (_array_element_2 _array_index_2) (`self.PickUpObjectsToRespawn`)
    (`KismetArrayLibrary.Array_Set` (`self.PickUpTransorms`) _array_index_2 (`self.GetTransform` _array_element_2) true)))

(fn `TriggerScript`
  (params (OverlappedComponent :type "PrimitiveComponent Object Reference") (OtherActor :type "Actor Object Reference") (OtherComp :type "PrimitiveComponent Object Reference") (OtherBodyIndex :type Integer) (bFromSweep :type Boolean) (SweepResult :type "HitResult Structure (by ref)"))
  (bind _asbp_game_mode (cast `/Game/Immersion_game/Core/BP_GameMode` (`GameplayStatics.GetGameMode`)))
  (set `/Game/Immersion_game/Core/BP_GameMode.LastCheckpoint` self _asbp_game_mode)
  (set `/Game/Immersion_game/Core/BP_GameMode.bHaveCheckpoint` true _asbp_game_mode)
  (return))

(fn `UserConstructionScript`
  (`parent.UserConstructionScript`))