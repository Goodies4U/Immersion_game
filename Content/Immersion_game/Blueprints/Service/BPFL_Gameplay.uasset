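; Gameplay function library with helpers for finding a drop location and turning a static mesh actor into a physics prop.
; DropLocation sphere-traces WorldStatic objects along an actor's forward vector, returning the hit point offset along its normal by the radius, or the trace end, with debug drawing enabled.
; DoPhysicalMesh makes the actor movable, ignores Pawn collision, assigns a valid mesh and passes that assignment's result to physics simulation.
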(fn `DoPhysicalMesh`
  (params (StaticMeshActor :type "StaticMeshActor Object Reference") (StaticMeshAsset :type "StaticMesh Object Reference"))
  (bind _staticmeshcomponent (`StaticMeshActor.StaticMeshComponent` StaticMeshActor))
  (`/Engine/EditorBlueprintResources/StandardMacros.IsValid` StaticMeshAsset
    (:`Is Valid`
      (`PrimitiveComponent.SetCollisionResponseToChannel` _staticmeshcomponent "ECC_Pawn" "ECR_Ignore")
      (`StaticMeshActor.SetMobility` StaticMeshActor "Movable")
      (bind _returnvalue (`StaticMeshComponent.SetStaticMesh` (`StaticMeshActor.StaticMeshComponent` StaticMeshActor) StaticMeshAsset))
      (`PrimitiveComponent.SetSimulatePhysics` _staticmeshcomponent _returnvalue))))

(fn `DropLocation`
  (params (DropFrom :type "Actor Object Reference") (TraceRadius :type "Float (double-precision)") (TraceDistance :type "Float (double-precision)"))
  (returns (ReturnLocation :type "Vector Structure"))
  (bind _returnvalue (`Actor.K2_GetActorLocation` DropFrom))
  (bind _outhit (`KismetSystemLibrary.SphereTraceSingleForObjects` null _returnvalue (+ _returnvalue (* (`Actor.GetActorForwardVector` DropFrom) TraceDistance)) (`local.TraceRadius`) (`|MakeArray` "ObjectTypeQuery1" :!type "EObjectTypeQuery Enum") false (`|MakeArray` DropFrom) "ForDuration"))
  (bind (_bblockinghit _binitialoverlap _time _distance _location _impactpoint _normal _impactnormal _physmat _hitactor _hitcomponent _hitbonename _bonename _hititem _elementindex _faceindex _tracestart _traceend) (`GameplayStatics.BreakHitResult` _outhit))
  (return (`KismetMathLibrary.SelectVector` (+ _impactpoint (* _impactnormal (`local.TraceRadius`))) _traceend _bblockinghit)))