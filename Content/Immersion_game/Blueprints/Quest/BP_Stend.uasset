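; BP_Stend is an interactable stand in the quest content that the player can step up to and view through the stand's own camera view.
; When the interaction trace hits its box, it shows a tooltip widget and a custom-depth outline on the banner.
; Starting interaction swaps to the minigame input context, blends the view, moves the character to the nearer side point and shows an input hint.
; The interaction key reverses this.
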(event `self.ReceiveBeginPlay`
  (`Widget.SetVisibility` (`WidgetComponent.GetWidget` (`self.BP_WidgetComp`)) "Collapsed"))

(event `/Game/Immersion_game/Blueprints/Interfaces/BPI_Interact.CancelCanInteract`
  (`self.ActivateOutlinerAndTooltip` false))

(event `/Game/Immersion_game/Blueprints/Interfaces/BPI_Interact.StopInteract`)

(event `EnhancedInput|/Game/Immersion_game/Inputs/Actions/Bool/IA_Interaction`
  (params (ActionValue :type Boolean) (ElapsedSeconds :type "Float (double-precision)") (TriggeredSeconds :type "Float (double-precision)") (InputAction :type "InputAction Object Reference" :default "/Game/Immersion_game/Inputs/Actions/Bool/IA_Interaction.IA_Interaction"))
  (bind _returnvalue (`GameplayStatics.GetPlayerController` 0))
  (bind _returnvalue_2 (pcsubsystem `EnhancedInputLocalPlayerSubsystem` (`GameplayStatics.GetPlayerController` 0)))
  (:`Started`
    (`EnhancedInputSubsystemInterface.RemoveMappingContext` _returnvalue_2 "/Game/Immersion_game/Inputs/IMC_MiniGame.IMC_MiniGame" (struct))
    (`EnhancedInputSubsystemInterface.AddMappingContext` _returnvalue_2 "/Game/Immersion_game/Inputs/IMC_Main.IMC_Main" 0 (struct))
    (set `/Game/Immersion_game/Blueprints/Components/BPC_Interact.bStopTraceCheck` false (`self.GetComponentByClass` (`GameplayStatics.GetPlayerCharacter` 0) "/Game/Immersion_game/Blueprints/Components/BPC_Interact.BPC_Interact_C"))
    (`PlayerController.SetViewTargetWithBlend` (`GameplayStatics.GetPlayerController` 0) (`GameplayStatics.GetPlayerCharacter` 0) 0.35 "VTBlend_Linear" 1.0 false)
    (`WidgetBlueprintLibrary.SetInputMode_GameOnly` _returnvalue)
    (`self.DisableInput` _returnvalue)
    (set `self.UseNow` false)
    (`Widget.RemoveFromParent` (`self.TutorialWidget`))))

(fn `ActivateOutlinerAndTooltip`
  (params (Active :type Boolean))
  (`Widget.SetVisibility` (`WidgetComponent.GetWidget` (`self.BP_WidgetComp`)) (select `bool` Active :`false` "Collapsed" :`true` "Visible" :!type "ESlateVisibility Enum"))
  (`PrimitiveComponent.SetRenderCustomDepth` (`self.NeskuchniyBanner`) Active))

(fn `CanInteract`
  (params (Hit :type "HitResult Structure") (QueryFromActor :type "Actor Object Reference"))
  (returns (True :type Boolean))
  (if (== (`.HitComponent` (`GameplayStatics.BreakHitResult` Hit)) (`self.Box`))
    (`self.ActivateOutlinerAndTooltip` true)
    (return true)
    (else
      (return false))))

(fn `MoveAndRotateCharacter`
  (bind _returnvalue (`GameplayStatics.GetPlayerController` 0))
  (bind _characterpositionleft (`self.CharacterPositionLeft`))
  (bind _characterpositionright (`self.CharacterPositionRight`))
  (bind _returnvalue_2 (`self.K2_GetActorLocation` (`GameplayStatics.GetPlayerCharacter` 0)))
  (bind (_returnvalue_roll _returnvalue_pitch) (`KismetMathLibrary.BreakRotator` (`self.K2_GetActorRotation` (`GameplayStatics.GetPlayerCharacter` 0))))
  (bind _returnvalue_3 (`SceneComponent.K2_GetComponentLocation` _characterpositionleft))
  (bind _returnvalue_4 (`SceneComponent.K2_GetComponentLocation` _characterpositionright))
  (bind _returnvalue_5 (< (`KismetMathLibrary.Vector_Distance` _returnvalue_2 _returnvalue_3) (`KismetMathLibrary.Vector_Distance` _returnvalue_2 _returnvalue_4)))
  (`AIBlueprintHelperLibrary.SimpleMoveToLocation` _returnvalue (`KismetMathLibrary.SelectVector` _returnvalue_3 _returnvalue_4 _returnvalue_5))
  (`Controller.SetControlRotation` _returnvalue (`KismetMathLibrary.MakeRotator` _returnvalue_roll _returnvalue_pitch (.yaw (`KismetMathLibrary.FindLookAtRotation` (`SceneComponent.K2_GetComponentLocation` (select `bool` _returnvalue_5 :`false` _characterpositionright :`true` _characterpositionleft)) (`SceneComponent.K2_GetComponentLocation` (`self.Box`)))))))

(fn `StartInteract`
  (params (InteractByActor :type "Actor Object Reference"))
  (returns (bSuccess :type Boolean) (bShouldPlayAnim :type Boolean) (bShouldRotateCharacterToObject :type Boolean))
  (bind _returnvalue (pcsubsystem `EnhancedInputLocalPlayerSubsystem` (`GameplayStatics.GetPlayerController` 0)))
  (if (not (`self.UseNow`))
    (`EnhancedInputSubsystemInterface.RemoveMappingContext` _returnvalue "/Game/Immersion_game/Inputs/IMC_Main.IMC_Main" (struct))
    (`EnhancedInputSubsystemInterface.AddMappingContext` _returnvalue "/Game/Immersion_game/Inputs/IMC_MiniGame.IMC_MiniGame" 0 (struct))
    (set `/Game/Immersion_game/Blueprints/Components/BPC_Interact.bStopTraceCheck` true (`self.GetComponentByClass` (`GameplayStatics.GetPlayerCharacter` 0) "/Game/Immersion_game/Blueprints/Components/BPC_Interact.BPC_Interact_C"))
    (`PlayerController.SetViewTargetWithBlend` (`GameplayStatics.GetPlayerController` 0) self 0.5 "VTBlend_Linear" 1.0 false)
    (set `self.UseNow` true)
    (`self.EnableInput` (`GameplayStatics.GetPlayerController` 0))
    (`self.MoveAndRotateCharacter`)
    (bind _returnvalue_2 (`|CreateWidget` "/Game/Immersion_game/UI/Service/W_Input.W_Input_C"))
    (bind _output_get (set `self.TutorialWidget` _returnvalue_2))
    (`UserWidget.AddToViewport` _output_get 0)
    (`self.ActivateOutlinerAndTooltip` false)
    (return true false false)))

(fn `UserConstructionScript`)