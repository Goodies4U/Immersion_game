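; BP_Puzzle is an interactable puzzle piece that rotates a quarter turn each time it is used.
; When it can be interacted with, it enables custom depth on its mesh and shows a prompt widget, hiding both when interaction is cancelled.
; StartInteract triggers a timeline that lerps the actor from its current rotation to the 90-degree offset, and rejects new interactions while that timeline plays.
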(event `self.ReceiveBeginPlay`
  (`Widget.SetVisibility` (`WidgetComponent.GetWidget` (`self.BP_WidgetComp`)) "Collapsed"))

(event `RotatePuzzle`
  (bind _rotation (`self.Rotation`))
  (set `self.Rotation` (`self.K2_GetActorRotation`))
  (bind (_direction _alpha) (`Timeline|RotateTimeline` :!via `PlayFromStart`)
    (:`Update`
      (`self.K2_SetActorRotation` (`KismetMathLibrary.RLerp` _rotation (`KismetMathLibrary.ComposeRotators` _rotation (struct :`Yaw` 90.0)) _alpha true)))))

(event `/Game/Immersion_game/Blueprints/Interfaces/BPI_Interact.CancelCanInteract`
  (`PrimitiveComponent.SetRenderCustomDepth` (`self.StaticMesh`) false)
  (`Widget.SetVisibility` (`WidgetComponent.GetWidget` (`self.BP_WidgetComp`)) "Collapsed"))

(fn `CanInteract`
  (returns (True :type Boolean))
  (`PrimitiveComponent.SetRenderCustomDepth` (`self.StaticMesh`) true)
  (`Widget.SetVisibility` (`WidgetComponent.GetWidget` (`self.BP_WidgetComp`)) "Visible")
  (return true))

(fn `StartInteract`
  (returns (bSuccess :type Boolean))
  (if (`TimelineComponent.IsPlaying` (`self.RotateTimeline`))
    (return false)
    (else
      (`self.RotatePuzzle`)
      (return true))))

(fn `UserConstructionScript`)