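; BP_SpawnStatueTrigger is a one-shot trigger actor that spawns statues at linked spawn points when overlapped.
; TriggerScript handles the overlap without filtering the other actor, calling DestroyActor on itself and then the SpawnStatueFromTrigger event.
; That event converts the SpawnPoints set to an array and calls SpawnStatue on each element.
; A disconnected copy of the same spawn loop remains in TriggerScript and never runs.
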(event `SpawnStatueFromTrigger`
  (if (`BlueprintSetLibrary.Set_IsNotEmpty` (`self.SpawnPoints`))
    (bind _result (`BlueprintSetLibrary.Set_ToArray` (`self.SpawnPoints`)))
    (for _array_element _result
      (`/Game/Immersion_game/Blueprints/Service/BP_StatueSpawner.SpawnStatue` _array_element))))

(fn `TriggerScript`
  (params (OverlappedComponent :type "PrimitiveComponent Object Reference") (OtherActor :type "Actor Object Reference") (OtherComp :type "PrimitiveComponent Object Reference") (OtherBodyIndex :type Integer) (bFromSweep :type Boolean) (SweepResult :type "HitResult Structure (by ref)"))
  (`self.K2_DestroyActor`)
  (`self.SpawnStatueFromTrigger`))

(fn `UserConstructionScript`)