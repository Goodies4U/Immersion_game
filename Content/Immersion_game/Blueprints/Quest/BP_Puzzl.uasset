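; Interactable puzzle station that switches the player into a mouse-driven minigame view.
; On interaction it swaps to the minigame input context, blends the camera to itself, walks the character to a set position and pauses interact tracing.
; Clicks trace from the cursor to trigger puzzle elements or other interactables; the interaction key restores normal play.
; While idle and targeted, it shows its widget and outlines all puzzle elements in the level.
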(event `self.ReceiveBeginPlay`
  (`Widget.SetVisibility` (`WidgetComponent.GetWidget` (`self.BP_WidgetComp`)) "Collapsed"))

(event `/Game/Immersion_game/Blueprints/Interfaces/BPI_Interact.CancelCanInteract`
  (`self.ActivateOutlinerAndTooltip` false))

(event `EnhancedInput|/Game/Immersion_game/Inputs/Actions/IA_SelectItem`
  (params (ActionValue :type Boolean) (ElapsedSeconds :type "Float (double-precision)") (TriggeredSeconds :type "Float (double-precision)") (InputAction :type "InputAction Object Reference" :default "/Game/Immersion_game/Inputs/Actions/IA_SelectItem.IA_SelectItem"))
  (bind (_worldlocation _worlddirection) (`PlayerController.DeprojectMousePositionToWorld` (`GameplayStatics.GetPlayerController` 0)))
  (:`Started`
    (bind (_outhit _returnvalue) (`KismetSystemLibrary.LineTraceSingle` :`Start` _worldlocation :`End` (+ _worldlocation (* _worlddirection 500.0)) :`TraceChannel` "TraceTypeQuery3" :`DrawDebugType` "ForDuration" :`DrawTime` 10.0))
    (if _returnvalue
      (bind (_bblockinghit _binitialoverlap _time _distance _location _impactpoint _normal _impactnormal _physmat _hitactor) (`GameplayStatics.BreakHitResult` _outhit))
      (if (== (`GameplayStatics.GetObjectClass` _hitactor) "/Game/Immersion_game/Blueprints/Quest/BP_PuzzleElement.BP_PuzzleElement_C")
        (message `/Game/Immersion_game/Blueprints/Interfaces/BPI_Interact.StartInteract` _hitactor null)
        (elif (`KismetSystemLibrary.DoesImplementInterface` _hitactor "/Game/Immersion_game/Blueprints/Interfaces/BPI_Interact.BPI_Interact_C")
          (message `/Game/Immersion_game/Blueprints/Interfaces/BPI_Interact.StartInteract` _hitactor (`GameplayStatics.GetPlayerCharacter` 0)))))))

(event `EnhancedInput|/Game/Immersion_game/Inputs/Actions/Bool/IA_Interaction`
  (params (ActionValue :type Boolean) (ElapsedSeconds :type "Float (double-precision)") (TriggeredSeconds :type "Float (double-precision)") (InputAction :type "InputAction Object Reference" :default "/Game/Immersion_game/Inputs/Actions/Bool/IA_Interaction.IA_Interaction"))
  (bind _returnvalue (`GameplayStatics.GetPlayerController` 0))
  (bind _returnvalue_2 (pcsubsystem `EnhancedInputLocalPlayerSubsystem` (`GameplayStatics.GetPlayerController` 0)))
  (:`Started`
    (`EnhancedInputSubsystemInterface.RemoveMappingContext` _returnvalue_2 "/Game/Immersion_game/Inputs/IMC_MiniGame.IMC_MiniGame" (struct))
    (`EnhancedInputSubsystemInterface.AddMappingContext` _returnvalue_2 "/Game/Immersion_game/Inputs/IMC_Main.IMC_Main" 0 (struct))
    (set `/Game/Immersion_game/Blueprints/Components/BPC_Interact.bStopTraceCheck` false (`self.GetComponentByClass` (`GameplayStatics.GetPlayerCharacter` 0) "/Game/Immersion_game/Blueprints/Components/BPC_Interact.BPC_Interact_C"))
    (`PlayerController.SetViewTargetWithBlend` (`GameplayStatics.GetPlayerController` 0) (`GameplayStatics.GetPlayerCharacter` 0) 0.35 "VTBlend_Linear" 1.0 false)
    (set `self.UseNow` false)
    (set `PlayerController.bShowMouseCursor` false _returnvalue)
    (`self.DisableInput` _returnvalue)
    (`WidgetBlueprintLibrary.SetInputMode_GameOnly` _returnvalue)))

(fn `ActivateOutlinerAndTooltip`
  (params (Active :type Boolean))
  (`Widget.SetVisibility` (`WidgetComponent.GetWidget` (`self.BP_WidgetComp`)) (select `bool` Active :`false` "Collapsed" :`true` "Visible" :!type "ESlateVisibility Enum"))
  (bind _outactors (`GameplayStatics.GetAllActorsOfClass` "/Game/Immersion_game/Blueprints/Quest/BP_PuzzleElement.BP_PuzzleElement_C"))
  (for _array_element _outactors
    (`/Game/Immersion_game/Blueprints/Quest/BP_PuzzleElement.ActivateOutliner` _array_element Active)))

(fn `CanInteract`
  (params (Hit :type "HitResult Structure") (QueryFromActor :type "Actor Object Reference"))
  (returns (True :type Boolean))
  (if (not (`self.UseNow`))
    (`self.ActivateOutlinerAndTooltip` true))
  (return true))

(fn `StartInteract`
  (params (InteractByActor :type "Actor Object Reference"))
  (returns (bSuccess :type Boolean) (bShouldPlayAnim :type Boolean) (bShouldRotateCharacterToObject :type Boolean))
  (bind _returnvalue (`GameplayStatics.GetPlayerController` 0))
  (bind _returnvalue_2 (pcsubsystem `EnhancedInputLocalPlayerSubsystem` (`GameplayStatics.GetPlayerController` 0)))
  (if (not (`self.UseNow`))
    (`EnhancedInputSubsystemInterface.RemoveMappingContext` _returnvalue_2 "/Game/Immersion_game/Inputs/IMC_Main.IMC_Main" (struct))
    (`EnhancedInputSubsystemInterface.AddMappingContext` _returnvalue_2 "/Game/Immersion_game/Inputs/IMC_MiniGame.IMC_MiniGame" 0 (struct))
    (set `/Game/Immersion_game/Blueprints/Components/BPC_Interact.bStopTraceCheck` true (`self.GetComponentByClass` (`GameplayStatics.GetPlayerCharacter` 0) "/Game/Immersion_game/Blueprints/Components/BPC_Interact.BPC_Interact_C"))
    (`PlayerController.SetViewTargetWithBlend` (`GameplayStatics.GetPlayerController` 0) self 0.5 "VTBlend_Linear" 1.0 false)
    (set `self.UseNow` true)
    (set `PlayerController.bShowMouseCursor` true _returnvalue)
    (`AIBlueprintHelperLibrary.SimpleMoveToLocation` _returnvalue (`SceneComponent.K2_GetComponentLocation` (`self.CharacterPosition`)))
    (`self.EnableInput` _returnvalue)
    (`WidgetBlueprintLibrary.SetInputMode_GameAndUIEx` _returnvalue null)
    (`self.ActivateOutlinerAndTooltip` false)
    (return true false false)))

(fn `UserConstructionScript`)