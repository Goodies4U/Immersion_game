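; BP_KeyHolder is a quest actor, named as a key holder, with two cube components that slide apart when its Open event is called.
; Open stores each cube's current relative location, then plays a timeline from the start.
; The timeline's alpha lerps the cubes to fixed offsets in opposite directions along local Y.
; Nothing in this Blueprint calls Open or closes the cubes again.
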(event `Open`
  (bind _relative_location_2 (`self.Relative Location 2`))
  (bind _relative_location_1 (`self.Relative Location 1`))
  (set `self.Relative Location 1` (`SceneComponent.RelativeLocation` (`self.Cube1`)))
  (set `self.Relative Location 2` (`SceneComponent.RelativeLocation` (`self.Cube2`)))
  (bind (_direction _alpha) (`Timeline|Timeline` :!via `PlayFromStart`)
    (:`Update`
      (`SceneComponent.K2_SetRelativeLocation` (`self.Cube1`) (`KismetMathLibrary.VLerp` _relative_location_1 (+ _relative_location_1 (0.0 -100.0 0.0)) _alpha) false false)
      (`SceneComponent.K2_SetRelativeLocation` (`self.Cube2`) (`KismetMathLibrary.VLerp` _relative_location_2 (+ _relative_location_2 (0.0 100.0 0.0)) _alpha) false false))))

(fn `UserConstructionScript`)