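; Base trigger Blueprint that reacts to living actors entering its collision component.
; On begin overlap, it finds the actor's float component tagged Health and calls TriggerScript, an empty hook for child classes, if that value is not zero.
; If ShouldDestroyAfterActivation is set, the trigger only flags itself Deactivated, since the DestroyComponent call is unconnected.
; Reactivate clears that flag so the trigger can fire again.
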(event `self.CollisionComponent.OnComponentBeginOverlap`
  (params (OverlappedComponent :type "PrimitiveComponent Object Reference") (OtherActor :type "Actor Object Reference") (OtherComp :type "PrimitiveComponent Object Reference") (OtherBodyIndex :type Integer) (bFromSweep :type Boolean) (SweepResult :type "HitResult Structure (by ref)"))
  (bind _returnvalue (`self.GetComponentsByTag` OtherActor "/Game/Immersion_game/Blueprints/Components/BPC_BaseFloatComponent.BPC_BaseFloatComponent_C" "Health"))
  (if (not (`self.bDeactivated`))
    (if (`KismetArrayLibrary.Array_IsNotEmpty` _returnvalue)
      (if (not (`/Game/Immersion_game/Blueprints/Components/BPC_BaseFloatComponent.GetValueEqualZero` (`|GetArrayItem` _returnvalue)))
        (`self.TriggerScript` OverlappedComponent OtherActor OtherComp OtherBodyIndex bFromSweep SweepResult)
        (if (`self.ShouldDestroyAfterActivation`)
          (set `self.bDeactivated` true))))))

(fn `Reactivate`
  (set `self.bDeactivated` false))

(fn `TriggerScript`
  (params (OverlappedComponent :type "PrimitiveComponent Object Reference") (OtherActor :type "Actor Object Reference") (OtherComp :type "PrimitiveComponent Object Reference") (OtherBodyIndex :type Integer) (bFromSweep :type Boolean) (SweepResult :type "HitResult Structure (by ref)"))
  (return))

(fn `UserConstructionScript`)