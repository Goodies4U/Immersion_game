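; Base interactable item actor that highlights itself and shows a tooltip widget when it can be interacted with.
; The construction script sets the mesh and tooltip icon from the item's data table row, and BeginPlay hides the tooltip and applies the physics setting.
; CanInteract and CancelCanInteract toggle custom depth and tooltip visibility.
; StartInteract gates InteractLogic behind CanInteract; InteractLogic is a stub returning failure, leaving behavior to overrides.
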(event `self.ReceiveBeginPlay`
  (`parent.ReceiveBeginPlay`)
  (`self.ToggleInteractFX` false)
  (`PrimitiveComponent.SetSimulatePhysics` (`self.Interactable`) (`self.bSimulatePhysics`)))

(event `self.CancelCanInteract`
  (`PrimitiveComponent.SetRenderCustomDepth` (`self.Interactable`) false)
  (`self.ToggleInteractFX` false))

(event `self.StopInteract`)

(fn `CanInteract`
  (params (Hit :type "HitResult Structure") (QueryFromActor :type "Actor Object Reference"))
  (returns (True :type Boolean))
  (`PrimitiveComponent.SetRenderCustomDepth` (`self.Interactable`) true)
  (`self.ToggleInteractFX` true)
  (return true))

(fn `InteractLogic`
  (params (InteractByActor :type "Actor Object Reference"))
  (returns (bSuccess :type Boolean) (bShouldPlayAnim :type Boolean) (bShouldRotateCharacterToObject :type Boolean))
  (return false false false))

(fn `StartInteract`
  (params (InteractByActor :type "Actor Object Reference"))
  (returns (bSuccess :type Boolean) (bShouldPlayAnim :type Boolean) (bShouldRotateCharacterToObject :type Boolean))
  (bind _true (`self.CanInteract` (struct) InteractByActor))
  (if _true
    (bind (_bsuccess _bshouldplayanim _bshouldrotatecharactertoobject) (`self.InteractLogic` InteractByActor))
    (if _bsuccess
      (return true _bshouldplayanim _bshouldrotatecharactertoobject)
      (else
        _)))
  (return false false false))

(fn `ToggleInteractFX`
  (params (bToggle :type Boolean))
  (bind _bp_widgetcomp (`self.BP_WidgetComp`))
  (bind _returnvalue (`WidgetComponent.GetWidget` _bp_widgetcomp))
  (`/Engine/EditorBlueprintResources/StandardMacros.IsValid` _bp_widgetcomp
    (:`Is Valid`
      (`/Engine/EditorBlueprintResources/StandardMacros.IsValid` _returnvalue
        (:`Is Valid`
          (`Widget.SetVisibility` _returnvalue (select `bool` bToggle :`false` "Collapsed" :`true` "Visible" :!type "ESlateVisibility Enum")))))))

(fn `UserConstructionScript`
  (bind _returnvalue (`self.GetItemObject`))
  (bind (_datatable _rowname) (break `DataTableRowHandle` (`ItemObjectCore.GetItemInfo` _returnvalue)))
  (`/Engine/EditorBlueprintResources/StandardMacros.IsValid` _returnvalue
    (:`Is Valid`
      (`/Engine/EditorBlueprintResources/StandardMacros.IsValid` _datatable
        (:`Is Valid`
          (bind _returnvalue_2 (`|GetDataTableRow` _datatable _rowname)
            (:`then`
              (bind ((`TooltipIcon` _tooltipicon) (`Model` _model)) (break `ItemInfo` _returnvalue_2))
              (`StaticMeshComponent.SetStaticMesh` (`self.Interactable`) _model)
              (set `/Game/Immersion_game/UI/Tooltip/BP_WidgetComp.Tool Tip Image` _tooltipicon (`self.BP_WidgetComp`)))
            (:`RowNotFound`
              (`StaticMeshComponent.SetStaticMesh` (`self.Interactable`) null :!label _label)
              (set `/Game/Immersion_game/UI/Tooltip/BP_WidgetComp.Tool Tip Image` null (`self.BP_WidgetComp`)))))
        (:`Is Not Valid`
          (goto _label))))))