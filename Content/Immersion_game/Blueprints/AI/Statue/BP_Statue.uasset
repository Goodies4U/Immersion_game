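; Statue character that shows wounds where it is hit and can play a paired StatueAttack action scene with another character.
; Face and Legs follow the Mesh pose; Mesh and Face each get a WoundComponent fed by a runtime-spawned scene capture.
; Point damage on Mesh picks face or body by physical material, using closest-physics-asset distance checks to spill nearby hits onto both.
; StartActionScene pairs the statue with any willing BPI_ActionScene character.
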(event `self.ReceiveBeginPlay`
  (`parent.ReceiveBeginPlay`)
  (`|ExecutionSequence`
    (:`then_0`
      (bind _returnvalue (`AddComponent|NODE_AddSceneCaptureComponent2D-1` :`RelativeTransform` (`KismetMathLibrary.MakeTransform` (0.0 0.0 250.0) (struct :`Pitch` -90.0 :`Yaw` 90.0 :`Roll` 180.0)))) ; There's some properties set in this node details panel
      (`SceneComponent.K2_AttachToComponent` _returnvalue (`self.Mesh`) "None" "SnapToTarget" "SnapToTarget" "SnapToTarget" true) ; This way even if you transform your mesh the scene capture still works
      (`/Game/Immersion_game/Blueprints/Components/WoundComponent.Initialize` (`self.WoundComponent1`) (`self.Face`) _returnvalue))
    (:`then_1`
      ;[1 1 1] Initialize the Components
      (bind _returnvalue_2 (`AddComponent|NODE_AddSceneCaptureComponent2D-0` :`RelativeTransform` (`KismetMathLibrary.MakeTransform` (0.0 0.0 250.0) (struct :`Pitch` -90.0 :`Yaw` 90.0 :`Roll` 180.0)))) ; There's some properties set in this node details panel
      (`SceneComponent.K2_AttachToComponent` _returnvalue_2 (`self.Mesh`) "None" "SnapToTarget" "SnapToTarget" "SnapToTarget" true) ; This way even if you transform your mesh the scene capture still works
      (`/Game/Immersion_game/Blueprints/Components/WoundComponent.Initialize` (`self.WoundComponent`) (`self.Mesh`) _returnvalue_2) ; Creates all the render targets and materials
    )))

(event `self.ReceivePointDamage`
  (params (Damage :type "Float (single-precision)") (DamageType :type "DamageType Object Reference") (HitLocation :type "Vector Structure") (HitNormal :type "Vector Structure") (HitComponent :type "PrimitiveComponent Object Reference") (BoneName :type Name) (ShotFromDirection :type "Vector Structure") (InstigatedBy :type "Controller Object Reference") (DamageCauser :type "Actor Object Reference") (HitInfo :type "HitResult Structure (by ref)"))
  (bind _returnvalue (* HitNormal -1.0))
  (bind _returnvalue_2 (select `bool` (`/Game/Immersion_game/Blueprints/Components/WoundComponent.UseProjectedWound` (`self.WoundComponent`)) :`false` (`KismetMathLibrary.RandomFloatInRange` 10.0 15.0) :`true` (`KismetMathLibrary.RandomFloatInRange` 3.0 5.0)))
  (set `self.NewVar` true)
  (if (== (`self.Mesh`) HitComponent)
    (if (== (`.PhysMat` (`GameplayStatics.BreakHitResult` HitInfo)) null)
      (`/Game/Immersion_game/Blueprints/Components/WoundComponent.TakeHit` (`self.WoundComponent1`) BoneName HitLocation _returnvalue _returnvalue_2 :!label _label)
      (if (`self.NewVar`)
        (if (< (`KismetMathLibrary.Vector_Distance` HitLocation (`SkeletalMeshComponent.K2_GetClosestPointOnPhysicsAsset` (`self.Mesh`) HitLocation)) 20.0)
          (set `self.NewVar` false)
          (`/Game/Immersion_game/Blueprints/Components/WoundComponent.TakeHit` (`self.WoundComponent`) BoneName HitLocation _returnvalue _returnvalue_2 :!label _label_2)
          (set `self.NewVar` (`self.NewVar`))
          (if (< (`KismetMathLibrary.Vector_Distance` HitLocation (`SkeletalMeshComponent.K2_GetClosestPointOnPhysicsAsset` (`self.Face`) HitLocation)) 20.0)
            (set `self.NewVar` false)
            (goto _label))))
      (else
        (goto _label_2)))))

(event `StartActionScene`
  (params (Character :type "Character Object Reference"))
  (bind _actionscene (`self.ActionScene`))
  (if (`KismetSystemLibrary.DoesImplementInterface` Character "/Game/Immersion_game/Blueprints/Components/PairAnimation/BPI_ActionScene.BPI_ActionScene_C")
    (bind _bsuccess (message `/Game/Immersion_game/Blueprints/Components/PairAnimation/BPI_ActionScene.CanBeInActionScene` Character))
    (if _bsuccess
      (message `/Game/Immersion_game/Blueprints/Components/PairAnimation/BPI_ActionScene.BindOnActionScene` Character _actionscene)
      (`/Game/Immersion_game/Blueprints/Components/PairAnimation/BPC_ActionScene.PairActionScene` _actionscene Character self (`self.StatueAttack`)))))

(fn `UserConstructionScript`
  (`parent.UserConstructionScript`)
  (`SkinnedMeshComponent.SetLeaderPoseComponent` (`self.Face`) (`self.Mesh`) false false)
  (`SkinnedMeshComponent.SetLeaderPoseComponent` (`self.Legs`) (`self.Mesh`) false false))