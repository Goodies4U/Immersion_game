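; Health pickup Blueprint that restores health to the actor interacting with it.
; It finds the actor's BPC_BaseFloatComponent tagged "Health" and, if not full, increases it by AddHealth, requesting an animation and rotation toward the object.
; CanInteract extends the parent check, allowing interaction only when that component exists and is not full.
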(fn `CanInteract`
  (params (Hit :type "HitResult Structure") (QueryFromActor :type "Actor Object Reference"))
  (returns (True :type Boolean))
  (bind _output (`|GetArrayItem` (`self.GetComponentsByTag` QueryFromActor "/Game/Immersion_game/Blueprints/Components/BPC_BaseFloatComponent.BPC_BaseFloatComponent_C" "Health")))
  (bind _true (`parent.CanInteract` Hit QueryFromActor))
  (`/Engine/EditorBlueprintResources/StandardMacros.IsValid` _output
    (:`Is Valid`
      (return (and _true (not (`/Game/Immersion_game/Blueprints/Components/BPC_BaseFloatComponent.GetValueFull` _output)))))
    (:`Is Not Valid`
      (return false))))

(fn `InteractLogic`
  (params (InteractByActor :type "Actor Object Reference"))
  (returns (bSuccess :type Boolean) (bShouldPlayAnim :type Boolean) (bShouldRotateCharacterToObject :type Boolean))
  (bind _output (`|GetArrayItem` (`self.GetComponentsByTag` InteractByActor "/Game/Immersion_game/Blueprints/Components/BPC_BaseFloatComponent.BPC_BaseFloatComponent_C" "Health")))
  (`/Engine/EditorBlueprintResources/StandardMacros.IsValid` _output
    (:`Is Valid`
      (if (not (`/Game/Immersion_game/Blueprints/Components/BPC_BaseFloatComponent.GetValueFull` _output))
        (`/Game/Immersion_game/Blueprints/Components/BPC_BaseFloatComponent.IncreaseValue` _output (`self.AddHealth`))
        (return true true true)
        (else
          _)))
    (:`Is Not Valid`
      _))
  (return false false false))

(fn `UserConstructionScript`
  (`parent.UserConstructionScript`))