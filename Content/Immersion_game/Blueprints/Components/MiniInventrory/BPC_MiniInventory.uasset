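; Mini inventory component for BP_Character, with one equipped item, one stowed slot and an array of non-equippable items.
; Data table rows behind each item object decide whether pickup spawns an actor attached to a mesh socket or stores the item.
; Toggling stows or re-equips with a montage; dropping spawns the pickup class at a traced location.
; ContainItem compares names but returns at the first entry with valid data.
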(event `self.ReceiveBeginPlay`
  (bind _asbp_character (cast `/Game/Immersion_game/Core/Character/BP_Character` (`self.GetOwner`)))
  (set `self.OwnerCharacter` _asbp_character))

(fn `ContainItem`
  (params (ItemName :type Name))
  (returns (bSuccess :type Boolean))
  (for _array_element (`self.InventoryArray`)
    (bind (_iteminfoproperties _bsuccess) (`self.Get Item Info` _array_element))
    (if _bsuccess
      (return (== (`.Name` (break `ItemInfo` _iteminfoproperties)) (`local.ItemName`)))))
  (return false))

(fn `DropItem`
  (returns (bSuccess :type Boolean))
  (bind _currentitem (`self.CurrentItem`)
    (:`then`
      (bind _returnvalue (`/Game/Immersion_game/Blueprints/Tools/BP_ParentTool.GetItemObject` _currentitem))
      (bind (_iteminfoproperties _bsuccess) (`self.Get Item Info` _returnvalue))
      (if _bsuccess
        (bind ((`ItemIcon` _itemicon) (`TooltipIcon` _tooltipicon) (`PickUpClass` _pickupclass) (`Model` _model)) (break `ItemInfo` _iteminfoproperties))
        (`|SpawnActorFromClass` _pickupclass (`KismetMathLibrary.MakeTransform` (`/Game/Immersion_game/Blueprints/Service/BPFL_Gameplay.DropLocation` (`self.GetOwner`) (`.SphereRadius` (`KismetMathLibrary.BreakBoxSphereBounds` (`StaticMesh.GetBounds` _model))) (`self.DropDistance`))) "AdjustIfPossibleButDontSpawnIfColliding" "OverrideRootScale" null _returnvalue null)
        (`Actor.K2_DestroyActor` (`self.CurrentItem`))
        (set `self.CurrentItem` null)
        (return true)
        (else
          _)))
    (:`else`
      _))
  (return false))

(fn `EquipItem`
  (params (ItemToEquip :type "ItemObjectCore Object Reference"))
  (returns (bSuccess :type Boolean))
  (`/Engine/EditorBlueprintResources/StandardMacros.IsValid` ItemToEquip
    (:`Is Valid`
      (`self.OwnerCharacter`
        (:`then`
          (`self.CurrentItem`
            (:`then`
              (return false))
            (:`else`
              (bind (_iteminfoproperties _bsuccess) (`self.Get Item Info` (`local.ItemToEquip`)))
              (if _bsuccess
                (bind ((`ItemIcon` _itemicon) (`TooltipIcon` _tooltipicon) (`EquipClass` _equipclass)) (break `ItemInfo` _iteminfoproperties))
                (if (`KismetSystemLibrary.IsValidClass` _equipclass)
                  (bind _returnvalue (`|SpawnActorFromClass` _equipclass (`KismetMathLibrary.MakeTransform` (0.0 0.0 0.0)) "Undefined" "OverrideRootScale" (`self.GetOwner`) (`local.ItemToEquip`) null))
                  (bind _output_get (set `self.CurrentItem` _returnvalue))
                  (`Actor.K2_AttachToComponent` _output_get (`Character.Mesh` (`self.OwnerCharacter`)) (`/Game/Immersion_game/Blueprints/Tools/BP_ParentTool.GetUseSocket` _output_get) "SnapToTarget" "SnapToTarget" "SnapToTarget" true)
                  (`self.OnEquip`)
                  (return true))
                (else
                  (return false))))))
        (:`else`
          (return false))))
    (:`Is Not Valid`
      (return false))))

(fn `Get Item Info`
  (params (ItemObject :type "ItemObjectCore Object Reference"))
  (returns (ItemInfoProperties :type "ItemInfo Structure") (bSuccess :type Boolean))
  (bind (_datatable _rowname) (break `DataTableRowHandle` (`ItemObjectCore.GetItemInfo` ItemObject)))
  (`/Engine/EditorBlueprintResources/StandardMacros.IsValid` _datatable
    (:`Is Valid`
      (bind _returnvalue (`|GetDataTableRow` _datatable _rowname)
        (:`then`
          (return _returnvalue true))
        (:`RowNotFound`
          _)))
    (:`Is Not Valid`
      _))
  (return (struct) false))

(fn `GetCurrentItem`
  (returns (CurrentItem :type "EquipClassCore Object Reference"))
  (return (`self.CurrentItem`)))

(fn `PickUpItem`
  (params (ObjectToPickUp :type "ItemObjectCore Object Reference"))
  (returns (bSuccess :type Boolean) (TimeToPickUp :type "Float (double-precision)"))
  (bind _objecttopickup (`local.ObjectToPickUp`))
  (bind (_iteminfoproperties _bsuccess) (`self.Get Item Info` ObjectToPickUp))
  (if _bsuccess
    (if (`KismetSystemLibrary.IsValidClass` (`.EquipClass` (break `ItemInfo` _iteminfoproperties)))
      (bind _bsuccess_2 (`self.EquipItem` _objecttopickup))
      (return _bsuccess_2 1.0)
      (else
        (`KismetArrayLibrary.Array_AddUnique` (`self.InventoryArray`) _objecttopickup)
        (return true 1.0)))))

(fn `ToggleItem`
  (returns (bSuccess :type Boolean))
  (bind _currentitem (`self.CurrentItem`))
  (bind _returnvalue (`EquipClassCore.GetItemObject` _currentitem))
  (`/Engine/EditorBlueprintResources/StandardMacros.IsValid` _currentitem
    (:`Is Valid`
      (`/Engine/EditorBlueprintResources/StandardMacros.IsValid` _returnvalue
        (:`Is Valid`
          (`self.ItemInBag`
            (:`then`
              _)
            (:`else`
              (`/Game/Immersion_game/Core/Character/BP_Character.PlayMontage` (cast `/Game/Immersion_game/Core/Character/BP_Character` (`GameplayStatics.GetPlayerCharacter` 0) :!pure true) null 2.0 false)
              (set `self.ItemInBag` _returnvalue)
              (`Actor.K2_DestroyActor` (`self.CurrentItem`))
              (`self.OnUnEquip`)
              (return true))))
        (:`Is Not Valid`
          _))
      (return false))
    (:`Is Not Valid`
      (`self.ItemInBag`
        (:`then`
          (bind _bsuccess (`self.EquipItem` (`self.ItemInBag`)))
          (if _bsuccess
            (`/Game/Immersion_game/Core/Character/BP_Character.PlayMontage` (cast `/Game/Immersion_game/Core/Character/BP_Character` (`GameplayStatics.GetPlayerCharacter` 0) :!pure true) null 2.0 false)
            (set `self.ItemInBag` null))
          (return _bsuccess))
        (:`else`
          (return false))))))