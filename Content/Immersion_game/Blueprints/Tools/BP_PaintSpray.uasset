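; Spray paint can tool that leaves paint decals on surfaces and damages actors tagged Enemy.
; Primary action start and stop toggle a muzzle Niagara effect, spray sounds and a fast looping timer.
; Paint traces randomly within a narrow cone, throttling enemy damage with a counter.
; Other hits get randomized, fading decals attached to the component, growing larger and fainter with distance.
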(fn `Initialization`
  (bind _returnvalue (`NiagaraFunctionLibrary.SpawnSystemAttached` "/Game/Immersion_game/VFX/NiagaraSystems/NS_Fire_Flamethrower.NS_Fire_Flamethrower" (`self.banka2`) "Muzzle" (0.0 0.0 0.0) (struct) "KeepRelativeOffset"))
  (bind _output_get (set `self.Niagara` _returnvalue))
  (`NiagaraComponent.SetVariableBool` _output_get "Active" false))

(fn `Paint`
  (locals (NewLocalVar :type Integer :default 6))
  (bind _banka2 (`self.banka2`))
  (bind _distance (`self.Distance`))
  (bind _returnvalue (`SceneComponent.GetSocketLocation` _banka2 "Muzzle"))
  (`/Engine/EditorBlueprintResources/StandardMacros.IncrementInt` (`self.Counter`)
    (:`  `
      (`|ExecutionSequence`
        (:`then_1`
          (bind (_outhit _returnvalue_2) (`KismetSystemLibrary.LineTraceSingleForObjects` :`Start` _returnvalue :`End` (+ _returnvalue (* (`KismetMathLibrary.RandomUnitVectorInConeInDegrees` (`KismetMathLibrary.GetForwardVector` (`SceneComponent.GetSocketRotation` _banka2 "Muzzle")) 8.0) (`self.Distance`))) :`ObjectTypes` (`|MakeArray` "ObjectTypeQuery1" "ObjectTypeQuery2" "ObjectTypeQuery1" :!type "EObjectTypeQuery Enum") :`DrawTime` 0.5))
          (if _returnvalue_2
            (bind (_bblockinghit _binitialoverlap _time _distance_2 _location _impactpoint _normal _impactnormal _physmat _hitactor _hitcomponent) (`GameplayStatics.BreakHitResult` _outhit))
            (if (`self.ActorHasTag` _hitactor "Enemy")
              (if (>= (`self.Counter`) 10)
                (`GameplayStatics.ApplyPointDamage` _hitactor 12.0 _location _outhit null (`self.GetOwner`) "/Script/Engine.DamageType")
                (set `self.Counter` 0))
              (else
                (bind _returnvalue_3 (`KismetMaterialLibrary.CreateDynamicMaterialInstance` (`|GetArrayItem` (`self.HorizontalDecals`) (`KismetMathLibrary.RandomIntegerInRange` 0 3))))
                (bind _returnvalue_4 (`KismetMathLibrary.Vector_Distance` (`SceneComponent.GetSocketLocation` (`self.banka2`) "Muzzle") _impactpoint))
                (`MaterialInstanceDynamic.SetScalarParameterValue` _returnvalue_3 "Opacity Intensity" (`KismetMathLibrary.MapRangeClamped` _returnvalue_4 0.0 _distance 0.2 0.01))
                (bind _returnvalue_5 (`GameplayStatics.SpawnDecalAttached` _returnvalue_3 (* (3.0 15.0 15.0) (`KismetMathLibrary.MapRangeClamped` _returnvalue_4 0.0 _distance 1.0 3.0)) _hitcomponent "None" _impactpoint (`KismetMathLibrary.MakeRotator` (.roll (`KismetMathLibrary.MakeRotFromX` _impactnormal)) (.pitch (`KismetMathLibrary.MakeRotFromX` _impactnormal)) (+ (.yaw (`KismetMathLibrary.MakeRotFromX` _impactnormal)) (`KismetMathLibrary.RandomFloatInRange` -90.0 90.0))) "KeepWorldPosition" 10.0))
                (`DecalComponent.SetFadeOut` _returnvalue_5 (`KismetMathLibrary.RandomFloatInRange` 10.0 20.0) (`KismetMathLibrary.RandomFloatInRange` 10.0 20.0) false)
                (`DecalComponent.SetFadeScreenSize` _returnvalue_5 0.005)))))))))

(fn `StartPrimaryActionLogic`
  (bind _niagara (`self.Niagara`)
    (:`then`
      (`NiagaraComponent.SetVariableBool` _niagara "Active" true)
      (bind _returnvalue (`KismetSystemLibrary.K2_SetTimerDelegate` (`|CreateDelegate` :!event `Paint`) 0.01 true))
      (set `self.TmerHande` _returnvalue)
      (bind _returnvalue_2 (`GameplayStatics.SpawnSoundAttached` "/Game/Resources/Sounds/SprayActive_Cue.SprayActive_Cue" (`self.banka2`) "None" (0.0 0.0 0.0) (struct) "KeepRelativeOffset" false 1.0 1.0 0.0 null null))
      (set `self.CurrentSound` _returnvalue_2))
    (:`else`)))

(fn `StopPrimaryActionLogic`
  (bind _niagara (`self.Niagara`)
    (:`then`
      (`NiagaraComponent.SetVariableBool` _niagara "Active" false)
      (`KismetSystemLibrary.K2_ClearAndInvalidateTimerHandle` (`self.TmerHande`))
      (`AudioComponent.Stop` (`self.CurrentSound`))
      (`GameplayStatics.SpawnSoundAttached` "/Game/Resources/Sounds/SprayEnd_Cue.SprayEnd_Cue" (`self.banka2`) "None" (0.0 0.0 0.0) (struct) "KeepRelativeOffset" false 1.0 1.0 0.0 null null))
    (:`else`)))

(fn `UserConstructionScript`
  (`parent.UserConstructionScript`))