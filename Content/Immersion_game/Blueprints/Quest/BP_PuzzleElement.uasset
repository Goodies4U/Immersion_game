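; Rotating puzzle piece that opens the BP_KeyHolder once every piece in the level shows its correct answer.
; A left-click trace or interact call plays a timeline turning the mesh 90 degrees and cycling its value through four states, starting from StartValue set at construction.
; After a correct turn, it polls all sibling pieces before triggering the holder.
; It supports custom-depth outlining and prints debug values every tick.
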(event `RotatePuzzle`
  (bind _rotation (`self.Rotation`))
  (bind _returnvalue (+ (`self.CurrentValue`) 1))
  (set `self.Rotation` (`SceneComponent.RelativeRotation` (`self.StaticMesh`)))
  (bind (_direction _alpha) (`Timeline|RotateTimeline` :!via `PlayFromStart`)
    (:`Update`
      (`SceneComponent.K2_SetRelativeRotation` (`self.StaticMesh`) (`KismetMathLibrary.RLerp` _rotation (`KismetMathLibrary.ComposeRotators` _rotation (struct :`Yaw` 90.0)) _alpha true) false false))
    (:`Finished`
      (set `self.CurrentValue` (`KismetMathLibrary.SelectInt` 0 _returnvalue (>= _returnvalue 4)))
      (if (== (`self.Answer`) (`self.CurrentValue`))
        (set `self.RightAnswer` true)
        (bind _outactors (`GameplayStatics.GetAllActorsOfClass` "BP_PuzzleElement_C"))
        (for _array_element _outactors
          (if (`/Game/Immersion_game/Blueprints/Quest/BP_PuzzleElement.RightAnswer` _array_element)
            (set `self.ShouldOpen` true)
            (else
              (set `self.ShouldOpen` false)
              (break))))
        (if (`self.ShouldOpen`)
          (`/Engine/EditorBlueprintResources/StandardMacros.DoOnce` false
            (:`Completed`
              (bind _returnvalue_2 (`GameplayStatics.GetActorOfClass` "/Game/Immersion_game/Blueprints/Quest/BP_KeyHolder.BP_KeyHolder_C"))
              (`/Game/Immersion_game/Blueprints/Quest/BP_KeyHolder.Open` _returnvalue_2))))
        (else
          (set `self.RightAnswer` false))))))

(event `Key|LeftMouseButton`
  (params (Key :type "Key Structure"))
  (bind (_worldlocation _worlddirection) (`PlayerController.DeprojectMousePositionToWorld` (`GameplayStatics.GetPlayerController` 0)))
  (:`Pressed`
    (bind (_outhit _returnvalue) (`KismetSystemLibrary.LineTraceSingle` :`Start` _worldlocation :`End` (+ _worldlocation (* _worlddirection 500.0)) :`TraceChannel` "TraceTypeQuery1" :`bIgnoreSelf` false :`DrawTime` 10.0))
    (if _returnvalue
      (if (== (`.HitComponent` (`GameplayStatics.BreakHitResult` _outhit)) (`self.StaticMesh`))
        (if (not (`TimelineComponent.IsPlaying` (`self.RotateTimeline`)))
          (`self.RotatePuzzle`))))))

(event `self.ReceiveTick`
  (params (DeltaSeconds :type "Float (single-precision)"))
  (`KismetSystemLibrary.PrintString` (`KismetTextLibrary.Conv_TextToString` (`|FormatText` "value{c}         answer{a}" (`self.CurrentValue`) (`self.Answer`))) true true (struct :`G` 1.0 :`B` 0.208507 :`A` 1.0) 0.0))

(fn `ActivateOutliner`
  (params (Active :type Boolean))
  (`PrimitiveComponent.SetRenderCustomDepth` (`self.StaticMesh`) Active))

(fn `CanInteract`
  (returns (True :type Boolean))
  (return true))

(fn `StartInteract`
  (params (InteractByActor :type "Actor Object Reference"))
  (returns (bSuccess :type Boolean))
  (if (not (`TimelineComponent.IsPlaying` (`self.RotateTimeline`)))
    (`self.RotatePuzzle`)
    (return true)))

(fn `UserConstructionScript`
  (bind _staticmesh (`self.StaticMesh`))
  (`SceneComponent.K2_SetRelativeRotation` _staticmesh (`KismetMathLibrary.ComposeRotators` (`SceneComponent.RelativeRotation` _staticmesh) (* (struct :`Yaw` 90.0) (`self.StartValue`))) false false)
  (set `self.CurrentValue` (`self.StartValue`)))