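; BP_MiniGames is an interactable mini-game actor that the player enters and exits through a StartInteract toggle.
; Entering swaps IMC_Main for the mini-game input context, pauses BPC_Interact tracing, walks the character to MoveToLocation and blends the view to this actor.
; IA_Interaction calls StartInteract again to exit, restoring input context, tracing and the character view.
; CheckNeedMouse optionally toggles cursor and input mode, while CanInteract blocks interaction during use.
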(event `EnhancedInput|/Game/Immersion_game/Inputs/Actions/Bool/IA_Interaction`
  (params (ActionValue :type Boolean) (ElapsedSeconds :type "Float (double-precision)") (TriggeredSeconds :type "Float (double-precision)") (InputAction :type "InputAction Object Reference" :default "/Game/Immersion_game/Inputs/Actions/Bool/IA_Interaction.IA_Interaction"))
  (:`Started`
    (`self.StartInteract` (`GameplayStatics.GetPlayerCharacter` 0))))

(fn `CanInteract`
  (params (Hit :type "HitResult Structure") (QueryFromActor :type "Actor Object Reference"))
  (returns (True :type Boolean))
  (if (not (`self.bUseNow`))
    (bind _true (`parent.CanInteract` Hit QueryFromActor))
    (return _true)
    (else
      (return false))))

(fn `CheckNeedMouse`
  (if (`self.bNeedMouse`)
    (if (`self.bUseNow`)
      (set `PlayerController.bShowMouseCursor` true (`GameplayStatics.GetPlayerController` 0))
      (`WidgetBlueprintLibrary.SetInputMode_GameAndUIEx` (`GameplayStatics.GetPlayerController` 0) null)
      (else
        (set `PlayerController.bShowMouseCursor` false (`GameplayStatics.GetPlayerController` 0))
        (`WidgetBlueprintLibrary.SetInputMode_GameOnly` (`GameplayStatics.GetPlayerController` 0))))))

(fn `GetUseNow`
  (returns (bUseNow :type Boolean))
  (return (`self.bUseNow`)))

(fn `SetUseNow`
  (params (bUseNow :type Boolean))
  (set `self.bUseNow` bUseNow))

(fn `StartInteract`
  (params (InteractByActor :type "Actor Object Reference"))
  (returns (bSuccess :type Boolean) (bShouldPlayAnim :type Boolean) (bShouldRotateCharacterToObject :type Boolean))
  (bind _returnvalue (`self.GetComponentByClass` (`GameplayStatics.GetPlayerCharacter` 0) "/Game/Immersion_game/Blueprints/Components/BPC_Interact.BPC_Interact_C"))
  (bind _returnvalue_2 (pcsubsystem `EnhancedInputLocalPlayerSubsystem` (`GameplayStatics.GetPlayerController` 0)))
  (if (`self.bUseNow`)
    (`EnhancedInputSubsystemInterface.RemoveMappingContext` _returnvalue_2 (`self.MiniGameInputContext`) (struct))
    (`EnhancedInputSubsystemInterface.AddMappingContext` _returnvalue_2 "/Game/Immersion_game/Inputs/IMC_Main.IMC_Main" 0 (struct))
    (set `/Game/Immersion_game/Blueprints/Components/BPC_Interact.bStopTraceCheck` false _returnvalue)
    (set `self.bUseNow` false)
    (`PlayerController.SetViewTargetWithBlend` (`GameplayStatics.GetPlayerController` 0) (`GameplayStatics.GetPlayerCharacter` 0) 0.1 "VTBlend_Linear" 1.0 false)
    (`self.CheckNeedMouse`)
    (`self.DisableInput` (`GameplayStatics.GetPlayerController` 0))
    (return true false false)
    (else
      (`EnhancedInputSubsystemInterface.RemoveMappingContext` _returnvalue_2 "/Game/Immersion_game/Inputs/IMC_Main.IMC_Main" (struct))
      (`EnhancedInputSubsystemInterface.AddMappingContext` _returnvalue_2 (`self.MiniGameInputContext`) 0 (struct))
      (set `/Game/Immersion_game/Blueprints/Components/BPC_Interact.bStopTraceCheck` true _returnvalue)
      (set `self.bUseNow` true)
      (`AIBlueprintHelperLibrary.SimpleMoveToLocation` (`GameplayStatics.GetPlayerController` 0) (`SceneComponent.K2_GetComponentLocation` (`self.MoveToLocation`)))
      (`PlayerController.SetViewTargetWithBlend` (`GameplayStatics.GetPlayerController` 0) self 0.1 "VTBlend_Linear" 1.0 false)
      (`self.EnableInput` (`GameplayStatics.GetPlayerController` 0))
      (`self.CheckNeedMouse`)
      (`self.ToggleInteractFX` false)
      (return true false false))))

(fn `ToggleInteractFX`
  (params (bToggle :type Boolean))
  (`parent.ToggleInteractFX` bToggle))

(fn `UserConstructionScript`
  (`parent.UserConstructionScript`))